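; Procedural dungeon generator that builds a level from room actors, following one of five random hard-coded sequences of normal, hub and shop rooms.
; After the start room, delayed spawns attach random rooms to the newest exit, tracking open exits and door points.
; Overlapping rooms are replaced at random exits, reloading the level once ten retries accumulate.
; Door, end-wall and timeout events exist but are uncalled here; computed special-room slots are unused.
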(event `Set Seeds`
  ;[0 0.05245 1] Set Seed
  (set `self.LayoutSeed` (`KismetMathLibrary.RandomInteger` 5))
  (bind _output_get (set `self.RoomSeed` (`KismetMathLibrary.RandomInteger` 1000)))
  (`KismetMathLibrary.SetRandomStreamSeed` (`self.Stream`) _output_get)
  (`self.Set Specials`))

(event `Start Dungeon Timer`
  ;[0 0.05245 1] Dungeon Failsafe
  (bind _returnvalue (`KismetSystemLibrary.K2_SetTimerDelegate` (delegate `Check Dungeon Completion`) 1.0 true))
  (set `self.Timer Handler` _returnvalue))

(event `Check Dungeon Completion`
  ;[0 0.05245 1] Dungeon Failsafe
  (if (>= (`KismetSystemLibrary.GetGameTimeInSeconds`) 20.0)
    (bind _returnvalue (`GameplayStatics.GetCurrentLevelName` true))
    (`GameplayStatics.OpenLevel` (`KismetStringLibrary.Conv_StringToName` _returnvalue))))

(event `self.ReceiveBeginPlay`
  ;[0 0.05245 1] Start Room Creation
  (`self.Set Seeds`)
  (`self.Spawn Start Room`)
  (`KismetSystemLibrary.Delay` 0.2)
  (`self.SpawnLayout`))

(event `SpawnLayout`
  ;[0 0.05245 1] Layout Spawner
  (switch `int` (`self.LayoutSeed`)
    (:`Default`
      (bind _returnvalue (`GameplayStatics.GetCurrentLevelName` true))
      (`GameplayStatics.OpenLevel` (`KismetStringLibrary.Conv_StringToName` _returnvalue)))
    (:`0`
      (`self.SpawnNormal`)
      (`KismetSystemLibrary.Delay` 0.2)
      (`self.SpawnNormal`)
      (`KismetSystemLibrary.Delay` 0.2)
      (`self.SpawnHub`)
      (`KismetSystemLibrary.Delay` 0.2)
      (`self.SpawnNormal`)
      (`KismetSystemLibrary.Delay` 0.2)
      (`self.SpawnNormal`)
      (`KismetSystemLibrary.Delay` 0.2)
      (`self.SpawnHub`)
      (`KismetSystemLibrary.Delay` 0.2)
      (`self.SpawnNormal`)
      (`KismetSystemLibrary.Delay` 0.2)
      (`self.SpawnNormal`)
      (`KismetSystemLibrary.Delay` 0.2)
      (`self.SpawnShop`))
    (:`1`
      (`self.SpawnNormal`)
      (`KismetSystemLibrary.Delay` 0.2)
      (`self.SpawnHub`)
      (`KismetSystemLibrary.Delay` 0.2)
      (`self.SpawnNormal`)
      (`KismetSystemLibrary.Delay` 0.2)
      (`self.SpawnNormal`)
      (`KismetSystemLibrary.Delay` 0.2)
      (`self.SpawnHub`)
      (`KismetSystemLibrary.Delay` 0.2)
      (`self.SpawnNormal`)
      (`KismetSystemLibrary.Delay` 0.2)
      (`self.SpawnNormal`)
      (`KismetSystemLibrary.Delay` 0.2)
      (`self.SpawnHub`)
      (`KismetSystemLibrary.Delay` 0.2)
      (`self.SpawnShop`))
    (:`2`
      (`self.SpawnHub`)
      (`KismetSystemLibrary.Delay` 0.2)
      (`self.SpawnNormal`)
      (`KismetSystemLibrary.Delay` 0.2)
      (`self.SpawnNormal`)
      (`KismetSystemLibrary.Delay` 0.2)
      (`self.SpawnNormal`)
      (`KismetSystemLibrary.Delay` 0.2)
      (`self.SpawnNormal`)
      (`KismetSystemLibrary.Delay` 0.2)
      (`self.SpawnHub`)
      (`KismetSystemLibrary.Delay` 0.2)
      (`self.SpawnNormal`)
      (`KismetSystemLibrary.Delay` 0.2)
      (`self.SpawnNormal`)
      (`KismetSystemLibrary.Delay` 0.2)
      (`self.SpawnShop`))
    (:`3`
      (`self.SpawnNormal`)
      (`self.SpawnNormal`)
      (`self.SpawnHub`)
      (`KismetSystemLibrary.Delay` 0.2)
      (`self.SpawnNormal`)
      (`KismetSystemLibrary.Delay` 0.2)
      (`self.SpawnNormal`)
      (`KismetSystemLibrary.Delay` 0.2)
      (`self.SpawnShop`)
      (`KismetSystemLibrary.Delay` 0.2)
      (`self.SpawnNormal`)
      (`KismetSystemLibrary.Delay` 0.2)
      (`self.SpawnNormal`)
      (`KismetSystemLibrary.Delay` 0.2)
      (`self.SpawnNormal`)
      (`KismetSystemLibrary.Delay` 0.2)
      (`self.SpawnHub`))
    (:`4`
      (`self.SpawnNormal`)
      (`self.SpawnNormal`)
      (`self.SpawnHub`)
      (`KismetSystemLibrary.Delay` 0.2)
      (`self.SpawnNormal`)
      (`KismetSystemLibrary.Delay` 0.2)
      (`self.SpawnNormal`)
      (`KismetSystemLibrary.Delay` 0.2)
      (`self.SpawnShop`)
      (`KismetSystemLibrary.Delay` 0.2)
      (`self.SpawnNormal`)
      (`KismetSystemLibrary.Delay` 0.2)
      (`self.SpawnNormal`)
      (`KismetSystemLibrary.Delay` 0.2)
      (`self.SpawnNormal`)
      (`KismetSystemLibrary.Delay` 0.2)
      (`self.SpawnHub`))))

(event `Spawn Start Room`
  ;[0 0.05245 1] Spawn Opening Room
  (bind _returnvalue (`|SpawnActorFromClass` "/Game/ProceduralRooms/Rooms/SpecialRooms/BP_StartRoom.BP_StartRoom_C" (`SceneComponent.K2_GetComponentToWorld` (`self.DefaultSceneRoot`)) "AlwaysSpawn" "MultiplyWithRoot" null null))
  (`self.RoomCounters` _returnvalue))

(event `Spawn Next Room`
  (params (RoomList :type "Array of Actor Class Reference (by ref)"))
  (bind _exits_list (`self.Exits List`))
  ;[0 0.05245 1] Spawn Next Room
  (bind _output_get (set `self.CurrentSelect` RoomList))
  (bind _output_get_2 (set `self.Selected Exit` (`|GetArrayItem` _exits_list (`.OutIndex` (`KismetArrayLibrary.Array_Random` _exits_list)))))
  (bind (_returnvalue_location _returnvalue_rotation) (`KismetMathLibrary.BreakTransform` (`SceneComponent.K2_GetComponentToWorld` _output_get_2)))
  (bind _returnvalue (`|SpawnActorFromClass` (`KismetArrayLibrary.Array_RandomFromStream` _output_get (`self.Stream`)) (`KismetMathLibrary.MakeTransform` _returnvalue_location _returnvalue_rotation) "AlwaysSpawn" "MultiplyWithRoot" null null))
  (bind _asbp_master_room (cast `/Game/ProceduralRooms/Rooms/BP_MasterRoom` _returnvalue))
  (set `self.LatestRoom` _asbp_master_room)
  (`KismetSystemLibrary.Delay` 0.2)
  (`self.Check for Overlap`))

(event `Spawn Fix Room`
  (params (RoomList :type "Array of Actor Class Reference (by ref)"))
  ;[0 0.05245 1] Fix Overlapping Rooms
  (bind _output_get (set `self.Selected Exit` (`KismetArrayLibrary.Array_Random` (`self.Exits List`))))
  (bind (_returnvalue_location _returnvalue_rotation) (`KismetMathLibrary.BreakTransform` (`SceneComponent.K2_GetComponentToWorld` _output_get)))
  (bind _returnvalue (`|SpawnActorFromClass` (`KismetArrayLibrary.Array_RandomFromStream` RoomList (`self.Stream`)) (`KismetMathLibrary.MakeTransform` _returnvalue_location _returnvalue_rotation) "AlwaysSpawn" "MultiplyWithRoot" null null))
  (bind _asbp_master_room (cast `/Game/ProceduralRooms/Rooms/BP_MasterRoom` _returnvalue))
  (set `self.LatestRoom` _asbp_master_room)
  (`KismetSystemLibrary.Delay` 0.2)
  (`self.RoomCounters` _asbp_master_room)
  (`self.Check for Overlap`))

(event `Add Overlappig Rooms`
  (bind _overlapbox (`/Game/ProceduralRooms/Rooms/BP_MasterRoom.OverlapBox` (`self.LatestRoom`)))
  ;[0 0.05245 1] Add for Overlapping Rooms
  (`KismetArrayLibrary.Array_Append` (`self.Overlapped List`) (`PrimitiveComponent.GetOverlappingComponents` _overlapbox))
  (for _array_element (`SceneComponent.GetChildrenComponents` _overlapbox false)
    (bind _asbox_collision (cast `BoxComponent` _array_element))
    (`KismetArrayLibrary.Array_Append` (`self.Overlapped List`) (`PrimitiveComponent.GetOverlappingComponents` _asbox_collision))))

(event `Check for Overlap`
  (bind _latestroom (`self.LatestRoom`))
  ;[0 0.05245 1] Check for Overlap
  (`self.Add Overlappig Rooms`)
  (if (`KismetArrayLibrary.Array_IsNotEmpty` (`self.Overlapped List`))
    (`KismetArrayLibrary.Array_Clear` (`self.Overlapped List`))
    (for _array_element (`SceneComponent.GetChildrenComponents` (`/Game/ProceduralRooms/Rooms/BP_MasterRoom.Exits` _latestroom) false)
      (`KismetArrayLibrary.Array_RemoveItem` (`self.Exits List`) _array_element))
    (`self.K2_DestroyActor` _latestroom)
    (bind _result (`/Engine/EditorBlueprintResources/StandardMacros.IncrementInt` (`self.OverlapCounter`))
      (:`  `
        (if (< _result 10)
          (`self.Spawn Fix Room ` (`self.CurrentSelect`))
          (else
            ;;[0 1 0.2814] Reset Level if No Exits
            (bind _returnvalue (`GameplayStatics.GetCurrentLevelName` true))
            (`GameplayStatics.OpenLevel` (`KismetStringLibrary.Conv_StringToName` _returnvalue))))))))

(event `Close Unused Exits`
  ;[0 0.05245 1] Close Unused Exits
  (for _array_element (`self.Exits List`)
    (bind (_returnvalue_location _returnvalue_rotation) (`KismetMathLibrary.BreakTransform` (`SceneComponent.K2_GetComponentToWorld` _array_element)))
    (`|SpawnActorFromClass` "/Game/ProceduralRooms/Rooms/BP_EndWall.BP_EndWall_C" (`KismetMathLibrary.MakeTransform` _returnvalue_location _returnvalue_rotation) "Undefined" "MultiplyWithRoot" null null)))

(event `Spawn Doors`
  ;[0 0.05245 1] Spawn Doors
  (for _array_element (`self.Door List`)
    (bind (_returnvalue_location _returnvalue_rotation) (`KismetMathLibrary.BreakTransform` (`SceneComponent.K2_GetComponentToWorld` _array_element)))
    (`|SpawnActorFromClass` "/Game/ProceduralRooms/Rooms/Doors/BP_Door.BP_Door_C" (`KismetMathLibrary.MakeTransform` _returnvalue_location _returnvalue_rotation) "AlwaysSpawn" "MultiplyWithRoot" null null)))

(fn `RandomFirstHalf`
  (returns (SpecialRoom :type Integer))
  (locals (RandomNumber :type Integer))
  (bind _randomnumber (`local.RandomNumber`))
  (bind _returnvalue (/ (`self.RoomAmount`) 2))
  (bind _returnvalue_2 (- (+ _returnvalue (`KismetMathLibrary.RandomIntegerInRange` 0 _returnvalue)) 3))
  (`KismetSystemLibrary.PrintString` (`KismetStringLibrary.Conv_IntToString` _returnvalue_2) true true (struct :`R` 0.21875 :`A` 1.0) 10.0)
  (bind _output_get (set `local.RandomNumber` _returnvalue_2))
  (if (== (mod _output_get 3) 0)
    (set `local.RandomNumber` (- (`local.RandomNumber`) 1))
    (return _randomnumber)
    (else
      (return _randomnumber))))

(fn `RandomLastHalf`
  (returns (`Special Num` :type Integer))
  (locals (RandomNumberGen :type Integer))
  (bind _randomnumbergen (`local.RandomNumberGen`))
  (bind _returnvalue (`KismetMathLibrary.RandomIntegerInRange` 2 (/ (`self.RoomAmount`) 2)))
  (`KismetSystemLibrary.PrintString` (`KismetStringLibrary.Conv_IntToString` _returnvalue) true true (struct :`G` 1.0 :`B` 0.281439 :`A` 1.0) 10.0)
  (bind _output_get (set `local.RandomNumberGen` _returnvalue))
  (if (== (mod _output_get 3) 0)
    (set `local.RandomNumberGen` (+ (`local.RandomNumberGen`) 2))
    (return _randomnumbergen)
    (else
      (return _randomnumbergen))))

(fn `RoomCounters`
  (params (SpawnedRoom :type "Actor Object Reference"))
  (bind _asbp_master_room (cast `/Game/ProceduralRooms/Rooms/BP_MasterRoom` SpawnedRoom))
  (set `self.LatestRoom` _asbp_master_room)
  (`/Engine/EditorBlueprintResources/StandardMacros.DecrementInt` (`self.RoomAmount`)
    (:`  `
      (`KismetArrayLibrary.Array_Add` (`self.Door List`) (`self.Selected Exit`))
      (`KismetArrayLibrary.Array_RemoveItem` (`self.Exits List`) (`self.Selected Exit`))
      (`KismetArrayLibrary.Array_Append` (`self.Exits List`) (`SceneComponent.GetChildrenComponents` (`/Game/ProceduralRooms/Rooms/BP_MasterRoom.Exits` (`self.LatestRoom`)) false)))))

(fn `Set Specials`
  (bind _specialnumbers (`self.SpecialNumbers`))
  (bind _speciallocations (`self.SpecialLocations`))
  (bind _specialnumbers_2 (`self.SpecialNumbers`))
  (bind _specialnumbers_3 (`self.SpecialNumbers`))
  (bind _output (`|GetArrayItem` _specialnumbers_3))
  (bind _output_2 (`|GetArrayItem` _specialnumbers_2 2))
  (bind _output_3 (`|GetArrayItem` _specialnumbers_2))
  (bind _output_4 (`|GetArrayItem` _specialnumbers_2 1))
  (bind _special_num (`self.RandomLastHalf`))
  (`KismetArrayLibrary.Array_Set` _specialnumbers 0 _special_num)
  (bind _specialroom (`self.RandomFirstHalf`))
  (`KismetArrayLibrary.Array_Set` _specialnumbers 1 _specialroom)
  (bind _special_num_2 (`self.RandomLastHalf`))
  (`KismetArrayLibrary.Array_Set` _specialnumbers 2 _special_num_2)
  (if (== _output (`|GetArrayItem` _specialnumbers_3 2))
    (`KismetArrayLibrary.Array_Set` _specialnumbers_2 0 (- _output 1))
    (if true
      (`KismetSystemLibrary.PrintText` (`|FormatText` "S: {S} 1:{1} 2: {2}" _output_3 _output_4 _output_2) true true (struct :`G` 0.66 :`B` 1.0 :`A` 1.0) 10.0 :!label _label)
      (`BlueprintMapLibrary.Map_Add` _speciallocations "Shop" _output_3)
      (`BlueprintMapLibrary.Map_Add` _speciallocations "Reward1" _output_4)
      (`BlueprintMapLibrary.Map_Add` _speciallocations "Reward2" _output_2))
    (else
      (goto _label))))

(fn `Spawn Special`
  (params (Rooms :type "Array of Actor Class Reference (by ref)")))

(fn `SpawnHub`
  (bind _rooms_hub (break `/Game/ProceduralRooms/S_Rooms` (`self.Rooms`)))
  (bind _exits_list (`self.Exits List`))
  (bind _output (`|GetArrayItem` _exits_list (`KismetArrayLibrary.Array_LastIndex` _exits_list)))
  (bind (_returnvalue_location _returnvalue_rotation) (`KismetMathLibrary.BreakTransform` (`SceneComponent.K2_GetComponentToWorld` _output)))
  (set `self.CurrentSelect` _rooms_hub)
  (set `self.Selected Exit` _output)
  (bind _returnvalue (`|SpawnActorFromClass` (`KismetArrayLibrary.Array_Random` _rooms_hub) (`KismetMathLibrary.MakeTransform` _returnvalue_location _returnvalue_rotation) "AlwaysSpawn" "MultiplyWithRoot" null null))
  (`self.RoomCounters` _returnvalue)
  (`self.Check for Overlap`))

(fn `SpawnNormal`
  (bind _normalrooms (`self.NormalRooms`))
  (bind _exits_list (`self.Exits List`))
  (bind _output (`|GetArrayItem` _exits_list (`KismetArrayLibrary.Array_LastIndex` _exits_list)))
  (bind (_returnvalue_location _returnvalue_rotation) (`KismetMathLibrary.BreakTransform` (`SceneComponent.K2_GetComponentToWorld` _output)))
  (set `self.CurrentSelect` _normalrooms)
  (set `self.Selected Exit` _output)
  (bind _returnvalue (`|SpawnActorFromClass` (`KismetArrayLibrary.Array_Random` _normalrooms) (`KismetMathLibrary.MakeTransform` _returnvalue_location _returnvalue_rotation) "AlwaysSpawn" "MultiplyWithRoot" null null))
  (`self.RoomCounters` _returnvalue)
  (`self.Check for Overlap`))

(fn `SpawnShop`
  (bind (_rooms_hub _rooms_shop) (break `/Game/ProceduralRooms/S_Rooms` (`self.Rooms`)))
  (bind _exits_list (`self.Exits List`))
  (bind _output (`|GetArrayItem` _exits_list (`KismetArrayLibrary.Array_LastIndex` _exits_list)))
  (bind (_returnvalue_location _returnvalue_rotation) (`KismetMathLibrary.BreakTransform` (`SceneComponent.K2_GetComponentToWorld` _output)))
  (set `self.CurrentSelect` _rooms_shop)
  (set `self.Selected Exit` _output)
  (bind _returnvalue (`|SpawnActorFromClass` (`KismetArrayLibrary.Array_Random` _rooms_shop) (`KismetMathLibrary.MakeTransform` _returnvalue_location _returnvalue_rotation) "AlwaysSpawn" "MultiplyWithRoot" null null))
  (`self.RoomCounters` _returnvalue)
  (`self.Check for Overlap`))

(fn `UserConstructionScript`)