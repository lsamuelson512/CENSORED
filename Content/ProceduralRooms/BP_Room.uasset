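; BP_Room builds a rectangular procedural room at BeginPlay, with instanced-mesh floor tiles and perimeter walls.
; WallOrDoor fills each edge slot with a wall instance or, at odd-indexed slots, possibly a spawned BP_Door, transformed from room-local space.
; Door odds use a random stream and shrink as Doors fills toward DoorCount.
; Non-origin rooms leave the first slot of the X=0 edge open.
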(event `self.ReceiveBeginPlay`
  (`self.BasicRoom`))

(fn `BasicRoom`
  ;[1 1 1] Generate Floor
  (for _index (range (`self.RoomTilesY`))
    (for _index_2 (range (`self.RoomTilesX`))
      (`InstancedStaticMeshComponent.AddInstance` (`self.Floor`) (`KismetMathLibrary.MakeTransform` (`KismetMathLibrary.MakeVector` (* _index_2 (`self.TileSizeX`)) (* (`self.TilseSizeY`) _index))) false)))
  ;[1 1 1] Walls
  (for _index_3 (range (`self.RoomTilesY`))
    (if (or (`self.OriginRoom`) (!= _index_3 0))
      (bind _returnvalue (== (mod _index_3 2) 1))
      (`self.WallOrDoor` _returnvalue (`KismetMathLibrary.MakeVector` 0.0 (* (`self.TilseSizeY`) _index_3)) (struct :`Yaw` 90.0)))
    (`self.WallOrDoor` _returnvalue (`KismetMathLibrary.MakeVector` (* (`self.RoomTilesX`) (`self.TileSizeX`)) (* (`self.TilseSizeY`) (+ _index_3 1))) (struct :`Yaw` -90.0)))
  (for _index_4 (range (`self.RoomTilesX`))
    (bind _returnvalue_2 (== (mod _index_4 2) 1))
    (`self.WallOrDoor` _returnvalue_2 (`KismetMathLibrary.MakeVector` (* (`self.TileSizeX`) _index_4) (* (`self.TilseSizeY`) (`self.RoomTilesY`))))
    (`self.WallOrDoor` _returnvalue_2 (`KismetMathLibrary.MakeVector` (* (`self.TileSizeX`) (+ _index_4 1))) (struct :`Yaw` 180.0))))

(fn `UserConstructionScript`)

(fn `WallOrDoor`
  (params (CanDoor :type Boolean) (InstanceTransformLocation :type "Vector Structure") (InstanceTransformRotation :type "Rotator Structure"))
  (bind _returnvalue (`self.GetTransform`))
  (bind _doorcount (`self.DoorCount`))
  ;[1 1 1] Door Check
  (if (and CanDoor (`KismetMathLibrary.RandomBoolWithWeightFromStream` (`self.Random Stream`) (/ (- _doorcount (`KismetArrayLibrary.Array_Length` (`self.Doors`))) _doorcount)))
    ;[1 1 1] Spawn Door
    (bind _returnvalue_2 (`|SpawnActorFromClass` "/Game/ProceduralRooms/BP_Door.BP_Door_C" (`KismetMathLibrary.MakeTransform` (`KismetMathLibrary.TransformLocation` _returnvalue InstanceTransformLocation) (`KismetMathLibrary.TransformRotation` _returnvalue InstanceTransformRotation)) "Undefined" "MultiplyWithRoot" null null))
    (`KismetArrayLibrary.Array_Add` (`self.Doors`) _returnvalue_2)
    (else
      ;[1 1 1] Spawn Wall
      (`InstancedStaticMeshComponent.AddInstance` (`self.Wall`) (`KismetMathLibrary.MakeTransform` InstanceTransformLocation InstanceTransformRotation) false))))