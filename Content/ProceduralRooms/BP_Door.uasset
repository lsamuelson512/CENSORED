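; BP_Door is a toggleable door that procedurally grows the level by spawning a new room when opened.
; Activate flips the Closed state and plays or reverses a timeline that drives the hinge's yaw.
; On the first opening only, a DoOnce calls NewRoom, which spawns a BP_Room ahead of the door with a rotation offset and randomized tile dimensions and door count.
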(event `/Game/ProceduralRooms/BPI_DoorActivate.Activate`
  (if (`self.Closed`)
    (set `self.Closed` false)
    (`|ExecutionSequence`
      (:`then_0`
        (`/Engine/EditorBlueprintResources/StandardMacros.DoOnce` false
          (:`Completed`
            (`self.NewRoom`))))
      (:`then_1`
        (bind (_direction _newtrack_0) (`Timeline|OpenDoorTimeline` :!label _label)
          (:`Update`
            (`SceneComponent.K2_SetRelativeRotation` (`self.Hinge`) (`KismetMathLibrary.MakeRotator` 0.0 0.0 _newtrack_0) false false)))))
    (else
      (set `self.Closed` true)
      (goto _label :!via `Reverse`))))

(event `NewRoom`
  (`|SpawnActorFromClass` "/Game/ProceduralRooms/BP_Room.BP_Room_C" (`KismetMathLibrary.MakeTransform` (+ (`self.K2_GetActorLocation`) (* (`self.GetActorForwardVector`) 400.0)) (`KismetMathLibrary.ComposeRotators` (`self.K2_GetActorRotation`) (struct :`Yaw` 90.0))) "Undefined" "MultiplyWithRoot" null (`KismetMathLibrary.RandomIntegerInRange` 3 6) (`KismetMathLibrary.RandomIntegerInRange` 3 6) (`KismetMathLibrary.RandomIntegerInRange` 1 4) null))

(fn `UserConstructionScript`)