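; Procedural dungeon generator that chains BP_MasterRoom actors onto open exits at level start.
; A seeded preset lays out the opening rooms, then random exits grow the dungeon with periodic hubs, two reward rooms and a final boss.
; Overlapping rooms and rewards near shops are destroyed and retried, with level reloads on repeated failure or timeout.
; Completion caps exits, adds doors, possesses enemies, places the player and lifts the black screen.
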(event `Set Seeds`
  ;[0 0.05245 1] Set Seed
  (set `self.LayoutSeed` (`KismetMathLibrary.RandomInteger` 5))
  (bind _output_get (set `self.RoomSeed` (`KismetMathLibrary.RandomInteger` 1000)))
  (`KismetMathLibrary.SetRandomStreamSeed` (`self.Stream`) _output_get)
  (`self.Set Specials`)
  (`self.SetLayout`))

(event `Start Dungeon Timer`
  ;[0 0.05245 1] Dungeon Failsafe
  (bind _returnvalue (`KismetSystemLibrary.K2_SetTimerDelegate` (delegate `Check Dungeon Completion`) 1.0 true))
  (set `self.Timer Handler` _returnvalue))

(event `Check Dungeon Completion`
  ;[0 0.05245 1] Dungeon Failsafe
  (if (>= (`KismetSystemLibrary.GetGameTimeInSeconds`) 20.0)
    (bind _returnvalue (`GameplayStatics.GetCurrentLevelName` true))
    (`GameplayStatics.OpenLevel` (`KismetStringLibrary.Conv_StringToName` _returnvalue))))

(event `self.ReceiveBeginPlay`
  ;[0 0.05245 1] Start Room Creation
  (`KismetSystemLibrary.Delay` 0.2)
  (`self.Set Seeds`)
  (`self.Spawn Start Room`)
  (`self.Start Dungeon Timer`)
  (`KismetSystemLibrary.Delay` 0.2)
  (`self.SpawnLayout`))

(event `Spawn Start Room`
  ;[0 0.05245 1] Spawn Opening Room
  (bind _returnvalue (`|SpawnActorFromClass` "/Game/ProceduralRooms/Rooms/SpecialRooms/BP_StartRoom.BP_StartRoom_C" (`SceneComponent.K2_GetComponentToWorld` (`self.DefaultSceneRoot`)) "AlwaysSpawn" "MultiplyWithRoot" null null))
  (`KismetArrayLibrary.Array_Append` (`self.Exits List`) (`SceneComponent.GetChildrenComponents` (`/Game/ProceduralRooms/Rooms/BP_MasterRoom.Exits` _returnvalue) false)))

(event `Spawn Next Room`
  (params (RoomList :type "Array of Actor Class Reference (by ref)"))
  ;[0 0.05245 1] Spawn Next Room
  (bind _output_get (set `self.CurrentSelect` RoomList))
  (bind _output_get_2 (set `self.Selected Exit` (`KismetArrayLibrary.Array_Random` (`self.Exits List`))))
  (bind (_returnvalue_location _returnvalue_rotation) (`KismetMathLibrary.BreakTransform` (`SceneComponent.K2_GetComponentToWorld` _output_get_2)))
  (bind _returnvalue (`|SpawnActorFromClass` (`KismetArrayLibrary.Array_RandomFromStream` _output_get (`self.Stream`)) (`KismetMathLibrary.MakeTransform` _returnvalue_location _returnvalue_rotation) "AlwaysSpawn" "MultiplyWithRoot" null null))
  (bind _asbp_master_room (cast `/Game/ProceduralRooms/Rooms/BP_MasterRoom` _returnvalue))
  (set `self.LatestRoom` _asbp_master_room)
  (`KismetSystemLibrary.Delay` 0.5)
  (`self.Check for Overlap`))

(event `FixOverlapLayout`
  (params (RoomList :type "Array of Actor Class Reference (by ref)"))
  ;[0 0.05245 1] Fix Overlapping Rooms Layout
  (bind _output_get (set `self.Selected Exit` (`KismetArrayLibrary.Array_Random` (`self.Exits List`))))
  (bind (_returnvalue_location _returnvalue_rotation) (`KismetMathLibrary.BreakTransform` (`SceneComponent.K2_GetComponentToWorld` _output_get)))
  (bind _returnvalue (`|SpawnActorFromClass` (`KismetArrayLibrary.Array_RandomFromStream` RoomList (`self.Stream`)) (`KismetMathLibrary.MakeTransform` _returnvalue_location _returnvalue_rotation) "AlwaysSpawn" "MultiplyWithRoot" null null))
  (bind _asbp_master_room (cast `/Game/ProceduralRooms/Rooms/BP_MasterRoom` _returnvalue))
  (set `self.LatestRoom` _asbp_master_room)
  (`KismetSystemLibrary.Delay` 0.2)
  (`self.Check for Overlap`))

(event `Spawn Fix Room`
  (params (RoomList :type "Array of Actor Class Reference (by ref)"))
  (bind _exits_list (`self.Exits List`))
  ;[0 0.05245 1] Fix Overlapping Rooms
  (bind _output_get (set `self.Selected Exit` (`|GetArrayItem` _exits_list (`.OutIndex` (`KismetArrayLibrary.Array_Random` _exits_list)))))
  (bind (_returnvalue_location _returnvalue_rotation) (`KismetMathLibrary.BreakTransform` (`SceneComponent.K2_GetComponentToWorld` _output_get)))
  (bind _returnvalue (`|SpawnActorFromClass` (`KismetArrayLibrary.Array_RandomFromStream` RoomList (`self.Stream`)) (`KismetMathLibrary.MakeTransform` _returnvalue_location _returnvalue_rotation) "AlwaysSpawn" "MultiplyWithRoot" null null))
  (bind _asbp_master_room (cast `/Game/ProceduralRooms/Rooms/BP_MasterRoom` _returnvalue))
  (set `self.LatestRoom` _asbp_master_room)
  (`KismetSystemLibrary.Delay` 0.2)
  (if (`self.Layout?`)
    (`self.CheckOverlapLayout`)
    (else
      (`self.Check for Overlap`))))

(event `CheckOverlapLayout`
  (bind _latestroom (`self.LatestRoom`))
  (bind _layoutindex (`self.LayoutIndex`))
  ;[0 0.05245 1] Check for Overlap Layout
  (`self.Add Overlappig Rooms`)
  (if (`KismetArrayLibrary.Array_IsNotEmpty` (`self.Overlapped List`))
    (`KismetArrayLibrary.Array_Clear` (`self.Overlapped List`))
    (for _array_element (`SceneComponent.GetChildrenComponents` (`/Game/ProceduralRooms/Rooms/BP_MasterRoom.Exits` _latestroom) false)
      (`KismetArrayLibrary.Array_RemoveItem` (`self.Exits List`) _array_element))
    (`self.K2_DestroyActor` _latestroom)
    (bind _result (`/Engine/EditorBlueprintResources/StandardMacros.IncrementInt` (`self.OverlapCounter`))
      (:`  `
        (if (< _result 10)
          (`self.Spawn Fix Room ` (`self.CurrentSelect`))
          (else
            ;;[0 1 0.2814] Reset Level if No Exits
            (bind _returnvalue (`GameplayStatics.GetCurrentLevelName` true))
            (`GameplayStatics.OpenLevel` (`KismetStringLibrary.Conv_StringToName` _returnvalue))))))
    (else
      (`self.Room Counters` (`self.LatestRoom`))
      (`/Engine/EditorBlueprintResources/StandardMacros.IncrementInt` _layoutindex
        (:`  `
          (`KismetSystemLibrary.Delay` 0.2)
          (`self.IncrementLayout` _layoutindex))))))

(event `Add Overlappig Rooms`
  (bind _overlapbox (`/Game/ProceduralRooms/Rooms/BP_MasterRoom.OverlapBox` (`self.LatestRoom`)))
  ;[0 0.05245 1] Add for Overlapping Rooms
  (`KismetArrayLibrary.Array_Append` (`self.Overlapped List`) (`PrimitiveComponent.GetOverlappingComponents` _overlapbox))
  (for _array_element (`SceneComponent.GetChildrenComponents` _overlapbox false)
    (bind _asbox_collision (cast `BoxComponent` _array_element))
    (`KismetArrayLibrary.Array_Append` (`self.Overlapped List`) (`PrimitiveComponent.GetOverlappingComponents` _asbox_collision))))

(event `Check for Overlap`
  (bind _roomamount (`self.RoomAmount`))
  (bind _speciallocations (`self.SpecialLocations`))
  (bind (_hub _shop _reward _boss) (break `/Game/ProceduralRooms/S_Rooms` (`self.Rooms`)))
  ;[0 0.05245 1] Check for Overlap
  (`self.Add Overlappig Rooms`)
  (if (`KismetArrayLibrary.Array_IsNotEmpty` (`self.Overlapped List`))
    (`KismetArrayLibrary.Array_Clear` (`self.Overlapped List`) :!label _label)
    (`self.K2_DestroyActor` (`self.LatestRoom`))
    (bind _result (`/Engine/EditorBlueprintResources/StandardMacros.IncrementInt` (`self.OverlapCounter`))
      (:`  `
        (if (< _result 10)
          (`self.Spawn Fix Room ` (`self.CurrentSelect`))
          (else
            ;;[0 1 0.2814] Reset Level if No Exits
            (bind _returnvalue (`GameplayStatics.GetCurrentLevelName` true :!label _label_2))
            (`GameplayStatics.OpenLevel` (`KismetStringLibrary.Conv_StringToName` _returnvalue))))))
    (else
      (if (`self.FoundSpecial`)
        (`self.RewardsCheck`
          (:`T`
            (goto _label))
          (:`F`
            _)))
      (`self.Room Counters` (`self.LatestRoom`))
      (if (`KismetArrayLibrary.Array_IsEmpty` (`self.Exits List`))
        (goto _label_2)
        (else
          (switch `int` _roomamount
            (:`Default`
              (if (== (mod _roomamount 15) 0)
                (`self.Spawn Next Room` _hub)
                (else
                  ;;[0 1 0.2814] Check Special Values
                  (bind _keys (`BlueprintMapLibrary.Map_Keys` _speciallocations))
                  (set `self.FoundSpecial` false)
                  (for _array_element _keys :!label _label_3
                    (if (== (`BlueprintMapLibrary.Map_Find` _speciallocations _array_element) (`self.RoomAmount`))
                      ;;[0 1 0.2814] If not shop, spawn reward
                      (set `self.FoundSpecial` true)
                      (`self.Spawn Next Room` _reward)))
                  ;;[0 1 0.2814] Special Value Not Found (Normal Room)
                  (if (not (`self.FoundSpecial`))
                    (`self.Spawn Next Room` (`self.NormalRooms`))))))
            (:`0`
              ;;[0 1 0.2814] Spawned All Rooms
              (`KismetSystemLibrary.K2_ClearAndInvalidateTimerHandle` (`self.Timer Handler`))
              (`self.Close Unused Exits`)
              (`self.Spawn Doors`)
              (`self.PossessEnemies` (`self.Enemies`))
              (`self.PlacePlayer`)
              (bind _asbp_hud (cast `/Game/Widgets/HUD/BP_HUD` (`PlayerController.GetHUD` (`GameplayStatics.GetPlayerController` 0))))
              (`/Game/Widgets/HUD/BP_HUD.RemoveBlackScreen` _asbp_hud))
            (:`1`
              ;;[0 1 0.2814] Final Room to Spawn (Boss)
              (`self.Spawn Next Room` _boss))))))))

(event `BreakLoop`
  ;[0 0.05245 1] Check for Overlap
  ;;[0 1 0.2814] Check Special Values
  (goto _label_3 :!via `Break`))

(event `Close Unused Exits`
  ;[0 0.05245 1] Close Unused Exits
  (for _array_element (`self.Exits List`)
    (bind (_returnvalue_location _returnvalue_rotation) (`KismetMathLibrary.BreakTransform` (`SceneComponent.K2_GetComponentToWorld` _array_element)))
    (`|SpawnActorFromClass` "/Game/ProceduralRooms/Rooms/DeadEnds/BP_DeadEnd.BP_DeadEnd_C" (`KismetMathLibrary.MakeTransform` _returnvalue_location _returnvalue_rotation) "AlwaysSpawn" "MultiplyWithRoot" null null)))

(event `Spawn Doors`
  ;[0 0.05245 1] Spawn Doors
  (for _array_element (`self.Door List`)
    (bind (_returnvalue_location _returnvalue_rotation) (`KismetMathLibrary.BreakTransform` (`SceneComponent.K2_GetComponentToWorld` _array_element)))
    (`|SpawnActorFromClass` "/Game/ProceduralRooms/Rooms/Doors/BP_Door.BP_Door_C" (`KismetMathLibrary.MakeTransform` _returnvalue_location _returnvalue_rotation) "AlwaysSpawn" "MultiplyWithRoot" null null)))

(event `SpawnLayout`
  ;[0 0.05245 1] Layout Spawner
  (`self.SpawnNormal` (`|GetArrayItem` (`self.StartingLayout`) (`self.LayoutIndex`))))

(fn `IncrementLayout`
  (params (A :type Integer))
  (if (<= A 8)
    (`self.SpawnLayout`)
    (else
      (set `self.Layout?` false)
      (`self.Spawn Next Room` (`self.NormalRooms`)))))

(fn `PlacePlayer`
  (bind _returnvalue (`GameplayStatics.GetActorOfClass` "/Script/Engine.PlayerStart"))
  (`self.K2_SetActorLocation` (`GameplayStatics.GetPlayerCharacter` 0) (`self.K2_GetActorLocation` _returnvalue) false false))

(fn `PossessEnemies`
  (params (`Array of Enemies` :type "Array of Actor Object Reference"))
  (for _array_element `Array of Enemies`
    (message `/Game/Enemies/BPI_EnemyActions.EnemyPosses` _array_element)))

(fn `RandomFirstHalf`
  (returns (SpecialRoom :type Integer))
  (locals (RandomNumber :type Integer))
  (bind _randomnumber (`local.RandomNumber`))
  (bind _returnvalue (/ (- (`self.RoomAmount`) 9) 2))
  (bind _output_get (set `local.RandomNumber` (+ _returnvalue (`KismetMathLibrary.RandomIntegerInRange` 0 _returnvalue))))
  (if (or (== (mod _output_get 15) 0) (== _output_get (`|GetArrayItem` (`self.SpecialNumbers`))))
    (set `local.RandomNumber` (- (`local.RandomNumber`) 1))
    (return _randomnumber)
    (else
      (return _randomnumber))))

(fn `RandomLastHalf`
  (returns (`Special Num` :type Integer))
  (locals (RandomNumberGen :type Integer))
  (bind _randomnumbergen (`local.RandomNumberGen`))
  (bind _output_get (set `local.RandomNumberGen` (`KismetMathLibrary.RandomIntegerInRange` 2 (/ (- (`self.RoomAmount`) 9) 2))))
  (if (== (mod _output_get 15) 0)
    (set `local.RandomNumberGen` (+ (`local.RandomNumberGen`) 2))
    (return _randomnumbergen)
    (else
      (return _randomnumbergen))))

(fn `Room Counters`
  (params (`Spawned Room` :type "Actor Object Reference"))
  (bind _latestroom (`self.LatestRoom`))
  (bind _asbp_master_room (cast `/Game/ProceduralRooms/Rooms/BP_MasterRoom` `Spawned Room`))
  (set `self.LatestRoom` _asbp_master_room)
  (`/Engine/EditorBlueprintResources/StandardMacros.DecrementInt` (`self.RoomAmount`)
    (:`  `
      (`KismetArrayLibrary.Array_Add` (`self.Door List`) (`self.Selected Exit`))
      (`KismetArrayLibrary.Array_RemoveItem` (`self.Exits List`) (`self.Selected Exit`))
      (`KismetArrayLibrary.Array_Append` (`self.Exits List`) (`SceneComponent.GetChildrenComponents` (`/Game/ProceduralRooms/Rooms/BP_MasterRoom.Exits` _latestroom) false))
      (`KismetArrayLibrary.Array_Append` (`self.Enemies`) (`self.GetAllChildActors` _latestroom true)))))

(fn `Set Specials`
  (bind _specialnumbers (`self.SpecialNumbers`))
  (bind _speciallocations (`self.SpecialLocations`))
  (bind _output (`|GetArrayItem` _specialnumbers 1))
  (bind _output_2 (`|GetArrayItem` _specialnumbers))
  (bind _special_num (`self.RandomLastHalf`))
  (`KismetArrayLibrary.Array_Set` _specialnumbers 0 _special_num)
  (bind _specialroom (`self.RandomFirstHalf`))
  (`KismetArrayLibrary.Array_Set` _specialnumbers 1 _specialroom)
  (`KismetSystemLibrary.PrintText` (`|FormatText` "LayoutSeed: {LS} \nR1:{1} R2: {2}" (`self.LayoutSeed`) _output_2 _output) true true (struct :`G` 0.66 :`B` 1.0 :`A` 1.0) 10.0)
  (`BlueprintMapLibrary.Map_Add` _speciallocations "Reward1" _output_2)
  (`BlueprintMapLibrary.Map_Add` _speciallocations "Reward2" _output))

(fn `SetLayout`
  (switch `int` (`self.LayoutSeed`)
    (:`Default`
      (bind _returnvalue (`GameplayStatics.GetCurrentLevelName` true))
      (`GameplayStatics.OpenLevel` (`KismetStringLibrary.Conv_StringToName` _returnvalue)))
    (:`0`
      (set `self.StartingLayout` (`|MakeArray` 0 0 1 0 0 1 0 0 2)))
    (:`1`
      (set `self.StartingLayout` (`|MakeArray` 0 1 0 0 1 0 0 0 2)))
    (:`2`
      (set `self.StartingLayout` (`|MakeArray` 1 0 0 1 0 0 0 0 2)))
    (:`3`
      (set `self.StartingLayout` (`|MakeArray` 0 1 0 0 2 0 0 0 1)))
    (:`4`
      (set `self.StartingLayout` (`|MakeArray` 0 1 0 0 2 0 0 0 1)))))

(fn `SpawnHub`
  (bind _rooms_hub (break `/Game/ProceduralRooms/S_Rooms` (`self.Rooms`)))
  (bind _exits_list (`self.Exits List`))
  (bind _output (`|GetArrayItem` _exits_list (`KismetArrayLibrary.Array_LastIndex` _exits_list)))
  (bind (_returnvalue_location _returnvalue_rotation) (`KismetMathLibrary.BreakTransform` (`SceneComponent.K2_GetComponentToWorld` _output)))
  (set `self.CurrentSelect` _rooms_hub)
  (set `self.Selected Exit` _output)
  (bind _returnvalue (`|SpawnActorFromClass` (`KismetArrayLibrary.Array_Random` _rooms_hub) (`KismetMathLibrary.MakeTransform` _returnvalue_location _returnvalue_rotation) "AlwaysSpawn" "MultiplyWithRoot" null null))
  (bind _asbp_master_room (cast `/Game/ProceduralRooms/Rooms/BP_MasterRoom` _returnvalue))
  (set `self.LatestRoom` _asbp_master_room)
  (`self.CheckOverlapLayout`))

(fn `SpawnNormal`
  (params (index :type Integer))
  (bind _exits_list (`self.Exits List`))
  (bind (_rooms_hub _rooms_shop _rooms_reward _rooms_boss) (break `/Game/ProceduralRooms/S_Rooms` (`self.Rooms`)))
  (bind _output (`|GetArrayItem` _exits_list (`KismetArrayLibrary.Array_LastIndex` _exits_list)))
  (bind (_returnvalue_location _returnvalue_rotation) (`KismetMathLibrary.BreakTransform` (`SceneComponent.K2_GetComponentToWorld` _output)))
  (bind _output_get (set `self.CurrentSelect` (select `int` index :`0` (`self.NormalRooms`) :`1` _rooms_hub :`2` _rooms_shop :`3` _rooms_boss)))
  (set `self.Selected Exit` _output)
  (bind _returnvalue (`|SpawnActorFromClass` (`KismetArrayLibrary.Array_Random` _output_get) (`KismetMathLibrary.MakeTransform` _returnvalue_location _returnvalue_rotation) "AlwaysSpawn" "MultiplyWithRoot" null null))
  (bind _asbp_master_room (cast `/Game/ProceduralRooms/Rooms/BP_MasterRoom` _returnvalue))
  (set `self.LatestRoom` _asbp_master_room)
  (`self.CheckOverlapLayout`))

(fn `SpawnShop`
  (bind (_rooms_hub _rooms_shop) (break `/Game/ProceduralRooms/S_Rooms` (`self.Rooms`)))
  (bind _exits_list (`self.Exits List`))
  (bind _output (`|GetArrayItem` _exits_list (`KismetArrayLibrary.Array_LastIndex` _exits_list)))
  (bind (_returnvalue_location _returnvalue_rotation) (`KismetMathLibrary.BreakTransform` (`SceneComponent.K2_GetComponentToWorld` _output)))
  (set `self.CurrentSelect` _rooms_shop)
  (set `self.Selected Exit` _output)
  (bind _returnvalue (`|SpawnActorFromClass` (`KismetArrayLibrary.Array_Random` _rooms_shop) (`KismetMathLibrary.MakeTransform` _returnvalue_location _returnvalue_rotation) "AlwaysSpawn" "MultiplyWithRoot" null null))
  (bind _asbp_master_room (cast `/Game/ProceduralRooms/Rooms/BP_MasterRoom` _returnvalue))
  (set `self.LatestRoom` _asbp_master_room)
  (`self.CheckOverlapLayout`))

(fn `UserConstructionScript`)