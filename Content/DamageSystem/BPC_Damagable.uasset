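; Actor component that gives its owner, apparently an enemy, health and handles taking damage and death.
; Damaged (always doubling its amount) and UnderlineDamage pass the ShouldDamage macro, which blocks only when both dead and invincible, then share one health check.
; Survivors print health and update the W_EnemyHealth widget.
; At zero, after a short delay, it raises the player's PlayWellBonus, calls KillChance on BPC_UniquePassives and destroys the owner.
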(event `Damaged`
  (params (DamageAmount :type "Float (double-precision)"))
  (bind _returnvalue (`Actor.GetComponentByClass` (`GameplayStatics.GetPlayerCharacter` 0) "/Game/Interactables/Items/GrabItems/BPC_UniquePassives.BPC_UniquePassives_C"))
  (`self.ShouldDamage`
    (:`Damage`
      (bind _output_get (set `self.Health` (- (`self.Health`) (`KismetMathLibrary.SelectFloat` DamageAmount (* DamageAmount 2.0)))))
      (if (<= _output_get 0.0) :!label _label
        (`KismetSystemLibrary.Delay` 0.2)
        (set `/Game/Interactables/Items/GrabItems/BPC_UniquePassives.PlayWellBonus` (+ (`/Game/Interactables/Items/GrabItems/BPC_UniquePassives.PlayWellBonus` _returnvalue) 0.01) _returnvalue)
        (`/Game/Interactables/Items/GrabItems/BPC_UniquePassives.KillChance` _returnvalue)
        (`Actor.K2_DestroyActor` (`self.GetOwner`))
        (else
          (`KismetSystemLibrary.PrintString` (`KismetStringLibrary.Conv_DoubleToString` _output_get))
          (`self.UpdateWidget`))))))

(event `UnderlineDamage`
  (`self.ShouldDamage`
    (:`Damage`
      (set `self.Health` (- (`self.Health`) (`self.Underline Dam`)))
      (goto _label))))

(fn `UpdateWidget`
  (bind _asw_enemy_health (cast `/Game/Widgets/Enemy/W_EnemyHealth` (`WidgetComponent.GetWidget` (`Actor.GetComponentByClass` (`self.GetOwner`) "/Script/UMG.WidgetComponent"))))
  (set `/Game/Widgets/Enemy/W_EnemyHealth.Health` (`self.Health`) _asw_enemy_health))