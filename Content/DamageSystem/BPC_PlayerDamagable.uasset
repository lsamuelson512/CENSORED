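; Player damage component that manages health, stat modifiers, revives and temporary invincibility.
; Damaged rolls through the ShouldDamage macro to ignore the hit, consume it as weapon ammo, block it or subtract health.
; UnderlineDamage skips those rolls, blocking only when dead and invincible, and shares the death check that spends a revive or destroys the owner.
; Timed events temporarily force full consume chance or invincibility; UpdateHealth applies the health modifier.
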(event `FullConsumption`
  (params (Duration :type "Float (single-precision)"))
  (bind (_mods_healthmod _mods_blockchance _mods_consumechance _mods_revives _mods_immunity) (break `/Game/Data/S_DamagableMods` (`self.Mods`)))
  (bind (_mods_healthmod_2 _mods_blockchance_2 _mods_consumechance_2 _mods_revives_2 _mods_immunity_2) (break `/Game/Data/S_DamagableMods` (`self.Mods`)))
  ;[0 0.05245 1] Full Consumption Back to Regular Amount
  (if (!= _mods_consumechance_2 1.0)
    (set `self.ConsumeChance` _mods_consumechance_2)
    (set `self.Mods` (make `/Game/Data/S_DamagableMods` _mods_healthmod_2 _mods_blockchance_2 1.0 _mods_revives_2 _mods_immunity_2))
    (`KismetSystemLibrary.Delay` Duration)
    (set `self.Mods` (make `/Game/Data/S_DamagableMods` _mods_healthmod _mods_blockchance (`self.ConsumeChance`) _mods_revives _mods_immunity))))

(event `UpdateHealth`
  (bind _mods_healthmod (break `/Game/Data/S_DamagableMods` (`self.Mods`)))
  (bind _returnvalue (* _mods_healthmod (`self.MaxHealth`)))
  ;[0 0.05245 1] Update Health
  (set `self.Health` (+ (- _returnvalue (`self.MaxHealth`)) (`self.Health`)))
  (set `self.MaxHealth` _returnvalue))

(event `Damaged`
  (params (DamageAmount :type "Float (double-precision)"))
  (bind (_mods_healthmod _mods_blockchance _mods_consumechance _mods_revives) (break `/Game/Data/S_DamagableMods` (`self.Mods`)))
  (bind (_mods_healthmod_2 _mods_blockchance_2 _mods_consumechance_2 _mods_revives_2) (break `/Game/Data/S_DamagableMods` (`self.Mods`)))
  ;[0 0.05245 1] Damage Check
  (`self.ShouldDamage`
    (:`Consume`
      (`self.Consume`))
    (:`Damage`
      (bind _output_get (set `self.Health` (- (`self.Health`) DamageAmount)))
      (if (<= _output_get 0.0) :!label _label
        (if (> _mods_revives 0)
          (`/Engine/EditorBlueprintResources/StandardMacros.DecrementInt` _mods_revives_2
            (:`  `
              (set `self.Revivable` false)
              (set `self.Health` (`self.MaxHealth`))))
          (else
            (`KismetSystemLibrary.Delay` 0.2)
            (`Actor.K2_DestroyActor` (`self.GetOwner`))))
        (else
          (`KismetSystemLibrary.PrintString` (`KismetStringLibrary.Conv_DoubleToString` _output_get)))))))

(event `UnderlineDamage`
  ;[0 0.05245 1] Damage Check
  (`self.ShouldUnderline`
    (:`Damage`
      (set `self.Health` (- (`self.Health`) (`self.UnderlineDam`)))
      (goto _label))))

(event `InvinciblePeroid`
  (params (Duration :type "Float (single-precision)"))
  (set `self.IsInvincible` true)
  (`KismetSystemLibrary.Delay` Duration)
  (set `self.IsInvincible` false))

(fn `Consume`
  (bind _returnvalue (`Actor.GetComponentByClass` (`self.GetOwner`) "/Game/FirstPerson/Blueprints/Weapons/BPC_PlayerWeapon.BPC_PlayerWeapon_C"))
  (`/Engine/EditorBlueprintResources/StandardMacros.IncrementInt` (`/Game/FirstPerson/Blueprints/Weapons/BPC_PlayerWeapon.CurrAmmo` _returnvalue)
    (:`  `
      (`/Game/FirstPerson/Blueprints/Weapons/BPC_PlayerWeapon.UpdateHUD` _returnvalue))))