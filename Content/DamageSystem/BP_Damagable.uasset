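; BP_Damagable is a component that tracks health for its owning actor and destroys that actor when health runs out.
; The Damaged event passes through the ShouldDamage gate, which blocks damage only when both IsDead and IsInvincible are true.
; Accepted damage reduces Health, then either prints the remaining value or destroys the owner after a short delay.
; IsDead is never set in these graphs.
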(event `Damaged`
  (params (DamageAmount :type "Float (double-precision)"))
  (`self.ShouldDamage`
    (:`Damage`
      (bind _output_get (set `self.Health` (- (`self.Health`) DamageAmount)))
      (if (<= _output_get 0.0)
        (`KismetSystemLibrary.Delay` 0.2)
        (`Actor.K2_DestroyActor` (`self.GetOwner`))
        (else
          (`KismetSystemLibrary.PrintString` (`KismetStringLibrary.Conv_DoubleToString` _output_get)))))))