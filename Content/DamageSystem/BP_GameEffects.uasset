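; BP_GameEffects manages text-formatting-themed status effects (Strikethrough, Bold, Italics, Underline) and reports them to its owner through messages.
; Strikethrough accumulates build-up, firing and resetting once it reaches a threshold.
; Bold and Italics toggle a damage-modifier message on and off, while Underline repeats a damage message through a delayed self-call loop.
; Retriggerable delays let repeated triggers refresh the timed effects' duration.
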(event `TriggerStrikethrough`
  (params (Additional :type "Float (double-precision)"))
  (bind _output_get (set `self.StrikethroughBuildUp` (+ Additional (`self.StrikethroughBuildUp`))))
  (if (>= _output_get 1.0)
    (message `/Game/DamageSystem/BPI_GameEffects.Strikethrough` (`self.GetOwner`))
    (set `self.StrikethroughBuildUp` 0.0)))

(event `TriggerBold`
  (set `self.Bold?` true)
  (message `/Game/DamageSystem/BPI_GameEffects.SetFxDamMod` (`self.GetOwner`) true true)
  (`KismetSystemLibrary.PrintString` "Bold")
  (`KismetSystemLibrary.RetriggerableDelay` (`self.Duration`))
  (set `self.Bold?` false)
  (message `/Game/DamageSystem/BPI_GameEffects.SetFxDamMod` (`self.GetOwner`) false true))

(event `TriggerItalics`
  (set `self.Italics?` true)
  (message `/Game/DamageSystem/BPI_GameEffects.SetFxDamMod` (`self.GetOwner`) true false)
  (`KismetSystemLibrary.PrintString` "Italics")
  (`KismetSystemLibrary.RetriggerableDelay` (`self.Duration`))
  (set `self.Italics?` false)
  (message `/Game/DamageSystem/BPI_GameEffects.SetFxDamMod` (`self.GetOwner`) false false))

(event `TriggerUnderline`
  (set `self.Underline?` true)
  (`self.UnderlineDamage`)
  (`KismetSystemLibrary.PrintString` "Underline")
  (`KismetSystemLibrary.RetriggerableDelay` (`self.Duration`))
  (set `self.Underline?` false))

(event `UnderlineDamage`
  (if (`self.Underline?`)
    (message `/Game/DamageSystem/BPI_GameEffects.UnderlineDamage` (`self.GetOwner`))
    (`KismetSystemLibrary.Delay` 0.5)
    (`self.UnderlineDamage`)))