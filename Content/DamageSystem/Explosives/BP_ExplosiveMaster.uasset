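; BP_ExplosiveMaster is an explosive actor that displays a randomly chosen command and deals area damage when detonated.
; On BeginPlay it picks from ExplosiveCommands and passes the text to its W_ExplosiveText widget, which yaws toward the player each Tick.
; Explode applies fixed damage through BPC_Damagable to Characters overlapping its Sphere, then destroys the actor after a short delay.
; Nothing in this graph calls Explode.
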(event `self.ReceiveBeginPlay`
  ;[0 0.05245 1] Select Command
  (set `self.SelectedCommand` (`KismetArrayLibrary.Array_Random` (`self.ExplosiveCommands`)))
  (bind _asw_explosive_text (cast `/Game/Widgets/Explosives/W_ExplosiveText` (`WidgetComponent.GetWidget` (`self.Widget`))))
  (set `/Game/Widgets/Explosives/W_ExplosiveText.TextCommand` (`self.SelectedCommand`) _asw_explosive_text))

(event `self.ReceiveTick`
  (params (DeltaSeconds :type "Float (single-precision)"))
  (bind _returnvalue (`GameplayStatics.GetPlayerCharacter` 0))
  (bind (_returnvalue_roll _returnvalue_pitch _returnvalue_yaw) (`KismetMathLibrary.BreakRotator` (`KismetMathLibrary.FindLookAtRotation` (`self.K2_GetActorLocation`) (`self.K2_GetActorLocation` _returnvalue))))
  ;[0 0.05245 1] Rotate Command to Face Actor
  (`/Engine/EditorBlueprintResources/StandardMacros.IsValid` _returnvalue
    (:`Is Valid`
      (`SceneComponent.K2_SetWorldRotation` (`self.Widget`) (`KismetMathLibrary.MakeRotator` 0.0 0.0 _returnvalue_yaw) false false))))

(event `Explode`
  ;[0 0.05245 1] Deal Damage
  (for _array_element (`PrimitiveComponent.GetOverlappingActors` (`self.Sphere`) "/Script/Engine.Character")
    (`/Game/DamageSystem/BPC_Damagable.Damaged` (`self.GetComponentByClass` _array_element "/Game/DamageSystem/BPC_Damagable.BPC_Damagable_C") 6.0))
  (`KismetSystemLibrary.Delay` 0.2)
  (`self.K2_DestroyActor`))

(fn `UserConstructionScript`)