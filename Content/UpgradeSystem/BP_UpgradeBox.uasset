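; BP_UpgradeBox is an interactable upgrade station where the player buys upgrades by typing their names.
; Box overlap toggles the HUD's interact widget and sets the first-person character's InteractCase.
; CheckText either closes the upgrade widget on the Esc command or matches committed text against DT_Upgrades names.
; The resulting row name goes to GI_PlayerStats' PurchaseUpgrade, then input focus returns to the prompt.
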(event `self.ReceiveBeginPlay`
  ;[0 0.05245 1] Creates ref to HUD
  (bind _asbp_hud (cast `/Game/Widgets/HUD/BP_HUD` (`PlayerController.GetHUD` (`GameplayStatics.GetPlayerController` 0))))
  (set `self.HUDRef` _asbp_hud))

(event `self.Box.OnComponentBeginOverlap`
  (params (OverlappedComponent :type "PrimitiveComponent Object Reference") (OtherActor :type "Actor Object Reference") (OtherComp :type "PrimitiveComponent Object Reference") (OtherBodyIndex :type Integer) (bFromSweep :type Boolean) (SweepResult :type "HitResult Structure (by ref)"))
  ;[0 0.05245 1] Add Interact Widget
  (if (== OtherActor (`GameplayStatics.GetPlayerCharacter` 0))
    (`UserWidget.AddToViewport` (`/Game/Widgets/HUD/BP_HUD.InteractRef` (`self.HUDRef`)) 0)
    (bind _asbp_first_person_character (cast `/Game/FirstPerson/Blueprints/BP_FirstPersonCharacter` (`GameplayStatics.GetPlayerCharacter` 0)))
    (set `/Game/FirstPerson/Blueprints/BP_FirstPersonCharacter.InteractCase` 1 _asbp_first_person_character)))

(event `self.Box.OnComponentEndOverlap`
  (params (OverlappedComponent :type "PrimitiveComponent Object Reference") (OtherActor :type "Actor Object Reference") (OtherComp :type "PrimitiveComponent Object Reference") (OtherBodyIndex :type Integer))
  ;[0 0.05245 1] Remove Interact Widget
  (if (== OtherActor (`GameplayStatics.GetPlayerCharacter` 0))
    (`Widget.RemoveFromParent` (`/Game/Widgets/HUD/BP_HUD.InteractRef` (`self.HUDRef`)))
    (bind _asbp_first_person_character (cast `/Game/FirstPerson/Blueprints/BP_FirstPersonCharacter` (`GameplayStatics.GetPlayerCharacter` 0)))
    (set `/Game/FirstPerson/Blueprints/BP_FirstPersonCharacter.InteractCase` 0 _asbp_first_person_character)))

(event `Check Text`
  (params (`Committed Text` :type Text))
  (bind _hudref (`self.HUDRef`))
  ;[0 0.05245 1] Check Text
  (if (== `Committed Text` (`self.Esc`))
    ;;[0 1 0.2814] Escape Command for Widget
    (`Widget.RemoveFromParent` (`/Game/Widgets/HUD/BP_HUD.UpgradeRef` _hudref))
    (`WidgetBlueprintLibrary.SetInputMode_GameOnly` (`GameplayStatics.GetPlayerController` 0))
    (`UserWidget.AddToViewport` (`/Game/Widgets/HUD/BP_HUD.InteractRef` _hudref) 0)
    (else
      ;;[0 1 0.2814] Check Upgrade
      (bind _rowname (`self.CheckUpgrade` `Committed Text`))
      (bind _output_get (set `self.SelectedRow` _rowname))
      (bind _asgi_player_stats (cast `/Game/SaveAndLoad/GI_PlayerStats` (`GameplayStatics.GetGameInstance`)))
      (`/Game/SaveAndLoad/GI_PlayerStats.PurchaseUpgrade` _asgi_player_stats _output_get)
      (`WidgetBlueprintLibrary.SetInputMode_UIOnlyEx` (`GameplayStatics.GetPlayerController` 0) (`/Game/Widgets/Upgrade/W_UpgradeMenu.Prompt` (`/Game/Widgets/HUD/BP_HUD.UpgradeRef` (`self.HUDRef`))) "LockAlways" true))))

(fn `CheckUpgrade`
  (params (CommittedText :type Text))
  (returns (RowName :type Name))
  (bind _outrownames (`DataTableFunctionLibrary.GetDataTableRowNames` "/Game/UpgradeSystem/DT_Upgrades.DT_Upgrades"))
  (for _array_element _outrownames
    (bind _returnvalue (`|GetDataTableRow` "/Game/UpgradeSystem/DT_Upgrades.DT_Upgrades" _array_element)
      (:`then`
        (if (== (`KismetTextLibrary.Conv_StringToText` (`|GetEnumeratorNameAsString` (`.Name_19_CFF0E8994D4444E50F40A39BFA385208` (break `/Game/UpgradeSystem/S_UpgradeInfo` _returnvalue)))) CommittedText)
          (return _array_element)))))
  (return "None"))

(fn `ItemPurchase`
  (params (ItemName :type Name))
  (returns (PurchasedItem :type Name))
  (return "None"))

(fn `UpgradePurchase`
  (params (UpgradeName :type Name))
  (returns (Upgrade :type "/Game/UpgradeSystem/E_Upgrades Enum"))
  (return "NewEnumerator39"))

(fn `UserConstructionScript`)