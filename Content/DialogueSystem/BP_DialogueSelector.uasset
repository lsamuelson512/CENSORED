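; BP_DialogueSelector is a possessable dialogue driver that steps through linked, voiced lines from a data table.
; On BeginPlay it attaches to the player character, plays the starting row, creates a pop-up widget referencing itself, and possesses itself after a short delay.
; Interact stops the current audio and advances via each row's NextLine index.
; At -1 it removes the widget and returns possession to the character.
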(event `EnhancedInput|/Game/FirstPerson/Input/Actions/IA_Interact`
  (params (ActionValue :type Boolean) (ElapsedSeconds :type "Float (double-precision)") (TriggeredSeconds :type "Float (double-precision)") (InputAction :type "InputAction Object Reference" :default "/Game/FirstPerson/Input/Actions/IA_Interact.IA_Interact"))
  (bind _lastaudio (`self.LastAudio`))
  (:`Started`
    (`/Engine/EditorBlueprintResources/StandardMacros.IsValid` _lastaudio
      (:`Is Valid`
        (`AudioComponent.Stop` _lastaudio))
      (:`Is Not Valid`
        _))
    (`self.NextDialogue`)))

(event `self.ReceiveBeginPlay`
  (bind _output_get (set `self.PlayerChar` (`GameplayStatics.GetPlayerCharacter` 0)))
  (`self.K2_AttachToActor` _output_get "None" "SnapToTarget" "SnapToTarget" "SnapToTarget")
  (bind _returnvalue (`|GetDataTableRow` (`self.DialogueDataTable`) (`KismetStringLibrary.Conv_StringToName` (`KismetStringLibrary.Conv_IntToString` (`self.StartingRow`))))
    (:`then`
      (set `self.DialogueRow` _returnvalue)
      (`self.NextDialogue`)
      (bind _returnvalue_2 (`|CreateWidget` "/Game/Widgets/Dialogue/W_DialoguePopUp.W_DialoguePopUp_C"))
      (bind _output_get_2 (set `self.DialogueWidgetRef` _returnvalue_2))
      (set `/Game/Widgets/Dialogue/W_DialoguePopUp.SelectorRef` self _output_get_2)
      (`UserWidget.AddToViewport` _output_get_2 0)
      (`KismetSystemLibrary.Delay` 0.4)
      (`Controller.Possess` (`GameplayStatics.GetPlayerController` 0) self))))

(event `NextDialogue`
  (bind (_dialoguerow_characterspeaking _dialoguerow_emotion _dialoguerow_dialogue _dialoguerow_sound _dialoguerow_nextline) (break `/Game/Data/Structs/S_Dialogue` (`self.DialogueRow`)))
  (bind (_dialoguerow_characterspeaking_2 _dialoguerow_emotion_2 _dialoguerow_dialogue_2 _dialoguerow_sound_2) (break `/Game/Data/Structs/S_Dialogue` (`self.DialogueRow`)))
  (bind (_dialoguerow_characterspeaking_3 _dialoguerow_emotion_3 _dialoguerow_dialogue_3 _dialoguerow_sound_3 _dialoguerow_nextline_2) (break `/Game/Data/Structs/S_Dialogue` (`self.DialogueRow`)))
  (if (== _dialoguerow_nextline_2 -1)
    (`Widget.RemoveFromParent` (`self.DialogueWidgetRef`))
    (`Controller.Possess` (`GameplayStatics.GetPlayerController` 0) (`self.PlayerChar`))
    (else
      (bind _returnvalue (`|GetDataTableRow` (`self.DialogueDataTable`) (`KismetStringLibrary.Conv_StringToName` (`KismetStringLibrary.Conv_IntToString` (`self.StartingRow`))))
        (:`then`
          (set `self.DialogueRow` _returnvalue)
          (bind _returnvalue_2 (`GameplayStatics.SpawnSound2D` _dialoguerow_sound_2 1.0 1.0 0.0 null))
          (set `self.LastAudio` _returnvalue_2)
          (set `self.StartingRow` _dialoguerow_nextline))))))

(fn `UserConstructionScript`)