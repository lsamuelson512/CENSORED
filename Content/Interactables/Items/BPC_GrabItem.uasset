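; Pickup component for item actors that grants stat modifiers or typed-command active items, logs the item name on the player, then destroys its owner.
; Separate functions additively stack weapon, bullet, player and damageable mods onto the first-person character and its components, with immunity flags OR-ed.
; Enemy mods stack on the BP_EnemySetter actor, and only the enemy damageable path calls UpdateBullet.
; Active items register their command and Blueprint with the typing-commands component.
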(fn `ActiveItem`
  (params (ItemInfo :type "/Game/Data/S_ItemInfo Structure"))
  (bind (_rarity _command _activeblueprint) (break `/Game/Data/S_ItemInfo` ItemInfo))
  (bind _asbp_first_person_character (cast `/Game/FirstPerson/Blueprints/BP_FirstPersonCharacter` (`GameplayStatics.GetPlayerPawn` 0)))
  (`/Game/FirstPerson/Blueprints/Weapons/TypingMechanics/BPC_TypingCommands.AddCommands` (`/Game/FirstPerson/Blueprints/BP_FirstPersonCharacter.BPC_TypingCommands` _asbp_first_person_character) _command _activeblueprint)
  (`KismetArrayLibrary.Array_Add` (`/Game/FirstPerson/Blueprints/BP_FirstPersonCharacter.Items` _asbp_first_person_character) (`self.ItemName`))
  (`Actor.K2_DestroyActor` (`self.GetOwner`)))

(fn `SetEnemyBulletMod`
  (params (BulletMod :type "/Game/Data/S_BulletMods Structure"))
  (bind (_strikethroughbuildup _italicsmod _underlinemod) (break `/Game/Data/S_BulletMods` BulletMod))
  (bind _returnvalue (`GameplayStatics.GetActorOfClass` "/Game/DamageSystem/BP_EnemySetter.BP_EnemySetter_C"))
  (bind (_bullet_mods_strikethroughbuildup _bullet_mods_italicsmod _bullet_mods_underlinemod) (break `/Game/Data/S_BulletMods` (`/Game/DamageSystem/BP_EnemySetter.Bullet Mods` _returnvalue)))
  (set `/Game/DamageSystem/BP_EnemySetter.Bullet Mods` (make `/Game/Data/S_BulletMods` (+ _bullet_mods_strikethroughbuildup _strikethroughbuildup) (+ _bullet_mods_italicsmod _italicsmod) (+ _bullet_mods_underlinemod _underlinemod)) _returnvalue)
  (bind _asbp_first_person_character (cast `/Game/FirstPerson/Blueprints/BP_FirstPersonCharacter` (`GameplayStatics.GetPlayerCharacter` 0)))
  (`KismetArrayLibrary.Array_Add` (`/Game/FirstPerson/Blueprints/BP_FirstPersonCharacter.Items` _asbp_first_person_character) (`self.ItemName`))
  (`Actor.K2_DestroyActor` (`self.GetOwner`)))

(fn `SetEnemyDamMod`
  (params (EnemyMod :type "/Game/Data/S_DamagableMods Structure"))
  (bind _returnvalue (`GameplayStatics.GetActorOfClass` "/Game/DamageSystem/BP_EnemySetter.BP_EnemySetter_C"))
  (bind (_enemymod_healthmod _enemymod_blockchance _enemymod_consumechance _enemymod_revives _enemymod_immunity) (break `/Game/Data/S_DamagableMods` (`/Game/DamageSystem/BP_EnemySetter.EnemyMod` _returnvalue)))
  (set `/Game/DamageSystem/BP_EnemySetter.EnemyMod` (make `/Game/Data/S_DamagableMods` (+ _enemymod_healthmod EnemyMod_HealthMod_10_BAE72AAB47FDF15064B0CEB1E799FD82) (+ _enemymod_blockchance EnemyMod_BlockChance_33_3A9512E0453265518B6485A3E232D618) (+ _enemymod_consumechance EnemyMod_ConsumeChance_36_3AA448AE4DBCC37D284C2982F208618B) 0 (or _enemymod_immunity EnemyMod_Immunity_14_51088F8647F1A26AA3E340B33C715AC5)) _returnvalue)
  (`/Game/DamageSystem/BP_EnemySetter.UpdateBullet` :`self` _returnvalue)
  (bind _asbp_first_person_character (cast `/Game/FirstPerson/Blueprints/BP_FirstPersonCharacter` (`GameplayStatics.GetPlayerCharacter` 0)))
  (`KismetArrayLibrary.Array_Add` (`/Game/FirstPerson/Blueprints/BP_FirstPersonCharacter.Items` _asbp_first_person_character) (`self.ItemName`))
  (`Actor.K2_DestroyActor` (`self.GetOwner`)))

(fn `SetPlayerBulletMod`
  (params (BulletMods :type "/Game/Data/S_BulletMods Structure"))
  (bind (_strikethroughbuildup _italicsmod _underlinemod) (break `/Game/Data/S_BulletMods` BulletMods))
  (bind _asbp_first_person_character (cast `/Game/FirstPerson/Blueprints/BP_FirstPersonCharacter` (`GameplayStatics.GetPlayerPawn` 0)))
  (bind _bp_weapon_component (`/Game/FirstPerson/Blueprints/BP_FirstPersonCharacter.BP_Weapon_Component` _asbp_first_person_character))
  (bind (_bulletmods_strikethroughbuildup _bulletmods_italicsmod _bulletmods_underlinemod) (break `/Game/Data/S_BulletMods` (`/Game/FirstPerson/Blueprints/Weapons/BPC_PlayerWeapon.BulletMods` _bp_weapon_component)))
  (set `/Game/FirstPerson/Blueprints/Weapons/BPC_PlayerWeapon.BulletMods` (make `/Game/Data/S_BulletMods` (+ _bulletmods_strikethroughbuildup _strikethroughbuildup) (+ _bulletmods_italicsmod _italicsmod) (+ _bulletmods_underlinemod _underlinemod)) _bp_weapon_component)
  (bind _asbp_first_person_character_2 (cast `/Game/FirstPerson/Blueprints/BP_FirstPersonCharacter` (`GameplayStatics.GetPlayerCharacter` 0)))
  (`KismetArrayLibrary.Array_Add` (`/Game/FirstPerson/Blueprints/BP_FirstPersonCharacter.Items` _asbp_first_person_character_2) (`self.ItemName`))
  (`Actor.K2_DestroyActor` (`self.GetOwner`)))

(fn `SetPlayerDamMod`
  (params (Mods :type "/Game/Data/S_DamagableMods Structure"))
  (bind (_healthmod _blockchance _consumechance _revives _immunity) (break `/Game/Data/S_DamagableMods` Mods))
  (bind _asbp_first_person_character (cast `/Game/FirstPerson/Blueprints/BP_FirstPersonCharacter` (`GameplayStatics.GetPlayerPawn` 0)))
  (`KismetArrayLibrary.Array_Add` (`/Game/FirstPerson/Blueprints/BP_FirstPersonCharacter.Items` _asbp_first_person_character) (`self.ItemName`))
  (bind _bp_playerdamagable (`/Game/FirstPerson/Blueprints/BP_FirstPersonCharacter.BP_PlayerDamagable` _asbp_first_person_character))
  (bind (_mods_healthmod _mods_blockchance _mods_consumechance _mods_revives _mods_immunity) (break `/Game/Data/S_DamagableMods` (`/Game/DamageSystem/BPC_PlayerDamagable.Mods` _bp_playerdamagable)))
  (set `/Game/DamageSystem/BPC_PlayerDamagable.Mods` (make `/Game/Data/S_DamagableMods` (+ _mods_healthmod _healthmod) (+ _mods_blockchance _blockchance) (+ _mods_consumechance _consumechance) (+ _mods_revives _revives) (or _mods_immunity _immunity)) _bp_playerdamagable)
  (`Actor.K2_DestroyActor` (`self.GetOwner`)))

(fn `SetPlayerMod`
  (params (PlayerMod :type "/Game/Data/S_PlayerMods Structure"))
  (bind _asbp_first_person_character (cast `/Game/FirstPerson/Blueprints/BP_FirstPersonCharacter` (`GameplayStatics.GetPlayerPawn` 0)))
  (bind (_playermod_typingtimemod _playermod_letterremoval _playermod_speedmod) (break `/Game/Data/S_PlayerMods` (`/Game/FirstPerson/Blueprints/BP_FirstPersonCharacter.PlayerMod` _asbp_first_person_character)))
  (set `/Game/FirstPerson/Blueprints/BP_FirstPersonCharacter.PlayerMod` (make `/Game/Data/S_PlayerMods` (+ _playermod_typingtimemod PlayerMod_TypingTimeMod_2_D66F9CFE42C8915A0AF8B48CE7CA515B) (+ _playermod_letterremoval PlayerMod_LetterRemoval_5_FEBFB79F44DAD57D06C283B9D2450C0E) (+ _playermod_speedmod PlayerMod_SpeedMod_8_C4E16CB14F1515CCD50A2AB719BD7C44)) _asbp_first_person_character)
  (`KismetArrayLibrary.Array_Add` (`/Game/FirstPerson/Blueprints/BP_FirstPersonCharacter.Items` _asbp_first_person_character) (`self.ItemName`))
  (`Actor.K2_DestroyActor` (`self.GetOwner`)))

(fn `SetWeaponMod`
  (params (DamagableMods :type "/Game/Data/S_WeaponMods Structure"))
  (bind _asbp_first_person_character (cast `/Game/FirstPerson/Blueprints/BP_FirstPersonCharacter` (`GameplayStatics.GetPlayerPawn` 0)))
  (`KismetArrayLibrary.Array_Add` (`/Game/FirstPerson/Blueprints/BP_FirstPersonCharacter.Items` _asbp_first_person_character) (`self.ItemName`))
  (bind _bp_weapon_component (`/Game/FirstPerson/Blueprints/BP_FirstPersonCharacter.BP_Weapon_Component` _asbp_first_person_character))
  (bind (_damagablemods_ammomod _damagablemods_damagemod _damagablemods_fireratemod) (break `/Game/Data/S_WeaponMods` (`/Game/FirstPerson/Blueprints/Weapons/BPC_PlayerWeapon.DamagableMods` _bp_weapon_component)))
  (set `/Game/FirstPerson/Blueprints/Weapons/BPC_PlayerWeapon.DamagableMods` (make `/Game/Data/S_WeaponMods` (+ _damagablemods_ammomod DamagableMods_AmmoMod_5_38F8A2EF405E66046BF5A0B5C51E918A) (+ _damagablemods_damagemod DamagableMods_DamageMod_9_80F6E31C4505A05798BFF9885A3215DA) (+ _damagablemods_fireratemod DamagableMods_FireRateMod_10_AB7D3E21446FAC1BF80BA8B3E29C53A2)) _bp_weapon_component)
  (`Actor.K2_DestroyActor` (`self.GetOwner`)))