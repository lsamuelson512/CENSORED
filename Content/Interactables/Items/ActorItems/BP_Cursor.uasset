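; BP_Cursor is an orbiting auto-turret that shoots at pawns it senses, ignoring the first player's pawn.
; Tick spins Gyro by Speed and places it and Cube around Scene at an offset scaled by Speed and Range, with no delta-time scaling.
; PawnSensing turns Cube toward the seen pawn, then after a short Delay spawns a BP_PistolProjectile from ProjectileSpawner and sets its damage.
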(event `self.PawnSensing.OnSeePawn`
  (params (Pawn :type "Pawn Object Reference"))
  (bind _projectilespawner (`self.ProjectileSpawner`))
  (bind (_returnvalue_roll _returnvalue_pitch _returnvalue_yaw) (`KismetMathLibrary.BreakRotator` (`KismetMathLibrary.FindLookAtRotation` (`SceneComponent.K2_GetComponentLocation` (`self.Cylinder`)) (`self.K2_GetActorLocation` Pawn))))
  (if (!= Pawn (`GameplayStatics.GetPlayerPawn` 0))
    (`SceneComponent.K2_SetWorldRotation` (`self.Cube`) (`KismetMathLibrary.MakeRotator` _returnvalue_roll _returnvalue_pitch _returnvalue_yaw) false false)
    (`KismetSystemLibrary.Delay` 0.2)
    (bind _returnvalue (`|SpawnActorFromClass` "/Game/FirstPerson/Blueprints/Weapons/Projectiles/BP_PistolProjectile.BP_PistolProjectile_C" (`KismetMathLibrary.MakeTransform` (`SceneComponent.K2_GetComponentLocation` _projectilespawner) (`SceneComponent.K2_GetComponentRotation` _projectilespawner)) "Undefined" "MultiplyWithRoot" null (struct) null))
    (set `/Game/FirstPerson/Blueprints/Weapons/Projectiles/BP_PistolProjectile.Damage` 0.75 _returnvalue)))

(event `self.ReceiveTick`
  (params (DeltaSeconds :type "Float (single-precision)"))
  (bind _gyro (`self.Gyro`))
  (bind (_relativerotation_roll _relativerotation_pitch _relativerotation_yaw) (`KismetMathLibrary.BreakRotator` (`SceneComponent.RelativeRotation` _gyro)))
  (`SceneComponent.K2_SetRelativeLocation` (`self.Gyro`) (+ (`SceneComponent.RelativeLocation` (`self.Scene`)) (* (`SceneComponent.GetRightVector` (`self.Gyro`)) (`self.Speed`) (`self.Range`))) false false)
  (`SceneComponent.K2_SetRelativeLocation` (`self.Cube`) (+ (`SceneComponent.RelativeLocation` (`self.Scene`)) (* (`SceneComponent.GetRightVector` (`self.Gyro`)) (`self.Speed`) (`self.Range`))) false false)
  (`SceneComponent.K2_SetRelativeRotation` _gyro (`KismetMathLibrary.MakeRotator` _relativerotation_roll _relativerotation_pitch (+ _relativerotation_yaw (`self.Speed`))) false false))

(fn `UserConstructionScript`)