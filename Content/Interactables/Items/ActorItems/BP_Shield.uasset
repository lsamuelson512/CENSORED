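; BP_Shield is a thrown shield projectile that ricochets between random actors from its enemies list, damaging what it hits.
; On spawn it launches at a fixed speed toward a random list entry.
; Each capsule overlap counts a bounce, deals fixed damage through BPC_Damagable if present, and redirects toward another random pick, which may repeat.
; An overlap after the bounce count exceeds MaxBounces destroys it instead.
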(event `self.ReceiveBeginPlay`
  ;[0 0.05245 1] Set Initial Velocity
  (set `MovementComponent.Velocity` (* (`KismetMathLibrary.GetForwardVector` (`KismetMathLibrary.FindLookAtRotation` (`self.K2_GetActorLocation`) (`self.K2_GetActorLocation` (`KismetArrayLibrary.Array_Random` (`self.EnemiesList`))))) 4000.0) (`self.ProjectileMovement`)))

(event `self.CollisionCapsule.OnComponentBeginOverlap`
  (params (OverlappedComponent :type "PrimitiveComponent Object Reference") (OtherActor :type "Actor Object Reference") (OtherComp :type "PrimitiveComponent Object Reference") (OtherBodyIndex :type Integer) (bFromSweep :type Boolean) (SweepResult :type "HitResult Structure (by ref)"))
  (bind _returnvalue (`self.GetComponentByClass` OtherActor "/Game/DamageSystem/BPC_Damagable.BPC_Damagable_C"))
  ;[0 0.05245 1] Bounce Between Targets
  (if (> (`self.Bounces`) (`self.MaxBounces`))
    (`self.K2_DestroyActor`)
    (else
      (`/Engine/EditorBlueprintResources/StandardMacros.IncrementInt` (`self.Bounces`)
        (:`  `
          (`/Engine/EditorBlueprintResources/StandardMacros.IsValid` _returnvalue
            (:`Is Valid`
              (`/Game/DamageSystem/BPC_Damagable.Damaged` _returnvalue 3.0))
            (:`Is Not Valid`
              _))
          (set `MovementComponent.Velocity` (* (`KismetMathLibrary.GetForwardVector` (`KismetMathLibrary.FindLookAtRotation` (`self.K2_GetActorLocation`) (`self.K2_GetActorLocation` (`KismetArrayLibrary.Array_Random` (`self.EnemiesList`))))) 4000.0) (`self.ProjectileMovement`)))))))

(fn `UserConstructionScript`)