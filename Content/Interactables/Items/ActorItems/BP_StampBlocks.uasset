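; BP_StampBlocks is a short-lived item actor that moves in a spinning circular motion and destroys itself ten seconds after BeginPlay.
; Each Tick sets the Gyro and Cube relative locations to the Scene's location, offset along the Gyro's right vector by Speed times Range.
; It then adds Speed to the Gyro's yaw, turning that offset into an orbit that is frame-rate dependent.
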(event `self.ReceiveBeginPlay`
  (`KismetSystemLibrary.Delay` 10.0)
  (`self.K2_DestroyActor`))

(event `self.ReceiveTick`
  (params (DeltaSeconds :type "Float (single-precision)"))
  (bind _gyro (`self.Gyro`))
  (bind (_relativerotation_roll _relativerotation_pitch _relativerotation_yaw) (`KismetMathLibrary.BreakRotator` (`SceneComponent.RelativeRotation` _gyro)))
  (`SceneComponent.K2_SetRelativeLocation` (`self.Gyro`) (+ (`SceneComponent.RelativeLocation` (`self.Scene`)) (* (`SceneComponent.GetRightVector` (`self.Gyro`)) (`self.Speed`) (`self.Range`))) false false)
  (`SceneComponent.K2_SetRelativeLocation` (`self.Cube`) (+ (`SceneComponent.RelativeLocation` (`self.Scene`)) (* (`SceneComponent.GetRightVector` (`self.Gyro`)) (`self.Speed`) (`self.Range`))) false false)
  (`SceneComponent.K2_SetRelativeRotation` _gyro (`KismetMathLibrary.MakeRotator` _relativerotation_roll _relativerotation_pitch (+ _relativerotation_yaw (`self.Speed`))) false false))

(fn `UserConstructionScript`)