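; Temporary turret item that shoots pistol projectiles at pawns it sees and destroys itself 30 seconds after spawning.
; PawnSensing reports sightings, and any pawn other than player 0's snaps the turret's yaw toward it.
; After a short Delay, which also limits the fire rate, it spawns BP_PistolProjectile at the ProjectileSpawner location along the turret's facing and overrides its damage.
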(event `self.ReceiveBeginPlay`
  (`ActorComponent.Activate` (`self.ProjectileSpawner`) false)
  (`KismetSystemLibrary.Delay` 30.0)
  (`self.K2_DestroyActor`))

(event `self.PawnSensing.OnSeePawn`
  (params (Pawn :type "Pawn Object Reference"))
  (bind (_returnvalue_roll _returnvalue_pitch _returnvalue_yaw) (`KismetMathLibrary.BreakRotator` (`KismetMathLibrary.FindLookAtRotation` (`self.K2_GetActorLocation`) (`self.K2_GetActorLocation` Pawn))))
  (if (!= Pawn (`GameplayStatics.GetPlayerPawn` 0))
    (`self.K2_SetActorRotation` (`KismetMathLibrary.MakeRotator` 0.0 0.0 _returnvalue_yaw))
    (`KismetSystemLibrary.Delay` 0.2)
    (bind _returnvalue (`|SpawnActorFromClass` "/Game/FirstPerson/Blueprints/Weapons/Projectiles/BP_PistolProjectile.BP_PistolProjectile_C" (`KismetMathLibrary.MakeTransform` (`SceneComponent.K2_GetComponentLocation` (`self.ProjectileSpawner`)) (`self.K2_GetActorRotation`)) "Undefined" "MultiplyWithRoot" null (struct) null))
    (set `/Game/FirstPerson/Blueprints/Weapons/Projectiles/BP_PistolProjectile.Damage` 0.75 _returnvalue)))

(fn `UserConstructionScript`)