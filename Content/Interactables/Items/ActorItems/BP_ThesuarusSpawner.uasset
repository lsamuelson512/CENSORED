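; Temporary actor that, despite its spawner name, controls infinite ammo through BPC_PlayerWeapon and spawns nothing.
; Its sphere turns InfiniteAmmo on when an actor with that component begins overlapping, and off when the overlap ends.
; On BeginPlay it waits on a fixed timer, forces infinite ammo on for the first player's pawn regardless of overlap, then destroys itself shortly afterwards.
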(event `self.ReceiveBeginPlay`
  (`KismetSystemLibrary.Delay` 10.0)
  (set `/Game/FirstPerson/Blueprints/Weapons/BPC_PlayerWeapon.InfiniteAmmo?` true (`self.GetComponentByClass` (`GameplayStatics.GetPlayerPawn` 0) "/Game/FirstPerson/Blueprints/Weapons/BPC_PlayerWeapon.BPC_PlayerWeapon_C"))
  (`KismetSystemLibrary.Delay` 0.2)
  (`self.K2_DestroyActor`))

(event `self.Sphere.OnComponentBeginOverlap`
  (params (OverlappedComponent :type "PrimitiveComponent Object Reference") (OtherActor :type "Actor Object Reference") (OtherComp :type "PrimitiveComponent Object Reference") (OtherBodyIndex :type Integer) (bFromSweep :type Boolean) (SweepResult :type "HitResult Structure (by ref)"))
  (bind _returnvalue (`self.GetComponentByClass` OtherActor "/Game/FirstPerson/Blueprints/Weapons/BPC_PlayerWeapon.BPC_PlayerWeapon_C"))
  (`/Engine/EditorBlueprintResources/StandardMacros.IsValid` _returnvalue
    (:`Is Valid`
      (set `/Game/FirstPerson/Blueprints/Weapons/BPC_PlayerWeapon.InfiniteAmmo?` true _returnvalue))))

(event `self.Sphere.OnComponentEndOverlap`
  (params (OverlappedComponent :type "PrimitiveComponent Object Reference") (OtherActor :type "Actor Object Reference") (OtherComp :type "PrimitiveComponent Object Reference") (OtherBodyIndex :type Integer))
  (bind _returnvalue (`self.GetComponentByClass` OtherActor "/Game/FirstPerson/Blueprints/Weapons/BPC_PlayerWeapon.BPC_PlayerWeapon_C"))
  (`/Engine/EditorBlueprintResources/StandardMacros.IsValid` _returnvalue
    (:`Is Valid`
      (set `/Game/FirstPerson/Blueprints/Weapons/BPC_PlayerWeapon.InfiniteAmmo?` false _returnvalue))))

(fn `UserConstructionScript`)