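; BP_ChampagneGlass is a unique item that trades a Glass state on the player for increased Mark gain.
; CommandCommit sets the Glass flag on the player's damageable component and adds a flat bonus to the economy component's MarkGainMod.
; Remove clears the flag and subtracts the same bonus, so the modifier is additive and reversible.
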(event `self.CommandCommit`
  (bind _playerref (`self.PlayerRef`))
  (bind _bpc_playereconomy (`/Game/FirstPerson/Blueprints/BP_FirstPersonCharacter.BPC_PlayerEconomy` _playerref))
  (set `/Game/DamageSystem/BPC_PlayerDamagable.Glass?` true (`/Game/FirstPerson/Blueprints/BP_FirstPersonCharacter.BP_PlayerDamagable` _playerref))
  (set `/Game/FirstPerson/Blueprints/Economy/BPC_PlayerEconomy.MarkGainMod` (+ (`/Game/FirstPerson/Blueprints/Economy/BPC_PlayerEconomy.MarkGainMod` _bpc_playereconomy) 0.5) _bpc_playereconomy))

(event `/Game/FirstPerson/Blueprints/Weapons/TypingMechanics/BPI_CommitText.Remove`
  (bind _playerref (`self.PlayerRef`))
  (bind _bpc_playereconomy (`/Game/FirstPerson/Blueprints/BP_FirstPersonCharacter.BPC_PlayerEconomy` _playerref))
  (set `/Game/DamageSystem/BPC_PlayerDamagable.Glass?` false (`/Game/FirstPerson/Blueprints/BP_FirstPersonCharacter.BP_PlayerDamagable` _playerref))
  (set `/Game/FirstPerson/Blueprints/Economy/BPC_PlayerEconomy.MarkGainMod` (+ (`/Game/FirstPerson/Blueprints/Economy/BPC_PlayerEconomy.MarkGainMod` _bpc_playereconomy) -0.5) _bpc_playereconomy))