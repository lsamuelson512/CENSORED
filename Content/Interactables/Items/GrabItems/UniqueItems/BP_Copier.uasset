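; BP_Copier is a unique grab item that doubles the player's mark gain while in effect.
; CommandCommit multiplies MarkGainMod on the player's BPCPlayerEconomy component by two, and Remove halves it to undo the boost.
; Both events scale the current value instead of setting it, so the bonus compounds with other changes to the modifier.
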(event `self.CommandCommit`
  (bind _bpc_playereconomy (`/Game/FirstPerson/Blueprints/BP_FirstPersonCharacter.BPC_PlayerEconomy` (`self.PlayerRef`)))
  (set `/Game/FirstPerson/Blueprints/Economy/BPC_PlayerEconomy.MarkGainMod` (* 2.0 (`/Game/FirstPerson/Blueprints/Economy/BPC_PlayerEconomy.MarkGainMod` _bpc_playereconomy)) _bpc_playereconomy))

(event `/Game/FirstPerson/Blueprints/Weapons/TypingMechanics/BPI_CommitText.Remove`
  (bind _bpc_playereconomy (`/Game/FirstPerson/Blueprints/BP_FirstPersonCharacter.BPC_PlayerEconomy` (`self.PlayerRef`)))
  (set `/Game/FirstPerson/Blueprints/Economy/BPC_PlayerEconomy.MarkGainMod` (* 0.5 (`/Game/FirstPerson/Blueprints/Economy/BPC_PlayerEconomy.MarkGainMod` _bpc_playereconomy)) _bpc_playereconomy))