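; Player character component that holds unique passive effects and abilities, including dash, stab and a self-repeating randomly timed Bold trigger.
; Kill and play bonuses register in maps that KillChance and PlayBonusChance scan to grant health, marks or Bold, with play bonuses rolled against PlayWellBonus.
; Count-limited dashes launch along movement input or opposite camera facing, optionally granting brief invincibility.
; Stab sphere-traces forward to damage BPC_Damagable actors, scaled by player modifiers.
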(event `ActivateKillBonus`
  (params (KillBonsActive :type "/Game/Data/E_KillBonuses Enum (by ref)"))
  ;[0 0.05245 1] Kill Bonus Action
  (`BlueprintMapLibrary.Map_Add` (`self.KillActive`) KillBonsActive true))

(event `RemoveKillBonus`
  (params (KillBonusActive :type "/Game/Data/E_KillBonuses Enum" :default "NewEnumerator0"))
  ;[0 0.05245 1] Remove Kill Bonus
  (`BlueprintMapLibrary.Map_Remove` (`self.KillActive`) KillBonusActive))

(event `self.ReceiveBeginPlay`
  ;[0 0.05245 1] Get Player Ref
  (bind _asbp_first_person_character (cast `/Game/FirstPerson/Blueprints/BP_FirstPersonCharacter` (`self.GetOwner`)))
  (set `self.PlayerRef` _asbp_first_person_character))

(event `ActivatePlayBonus`
  (params (PlayBonusActive :type "/Game/Data/E_PlayBonuses Enum" :default "NewEnumerator0"))
  ;[0 0.05245 1] Play Bonus Activation
  (`BlueprintMapLibrary.Map_Add` (`self.PlayBonusActive`) PlayBonusActive true))

(event `RandomBold`
  ;[0 0.05245 1] Random Bold
  (`KismetSystemLibrary.Delay` (`KismetMathLibrary.RandomFloatInRange` 120.0 240.0))
  (`/Game/DamageSystem/BPC_GameEffects.TriggerBold` (`Actor.GetComponentByClass` (`self.GetOwner`) "/Game/DamageSystem/BPC_GameEffects.BPC_GameEffects_C"))
  (`self.RandomBold`))

(event `EnhancedInput|/Game/FirstPerson/Input/Actions/IA_Dash`
  (params (ActionValue :type Boolean) (ElapsedSeconds :type "Float (double-precision)") (TriggeredSeconds :type "Float (double-precision)") (InputAction :type "InputAction Object Reference" :default "/Game/FirstPerson/Input/Actions/IA_Dash.IA_Dash"))
  (bind _playerref (`self.PlayerRef`))
  (bind (_playermod_typingtimemod _playermod_letterremoval _playermod_speedmod _playermod_dashmod) (break `/Game/Data/Structs/S_PlayerMods` (`/Game/FirstPerson/Blueprints/BP_FirstPersonCharacter.PlayerMod` (`self.PlayerRef`))))
  (bind _returnvalue (* (`Pawn.GetLastMovementInputVector` _playerref) 3000.0 _playermod_dashmod))
  ;[0 0.05245 1] Dash Ability
  (:`Started`
    (if (> (`self.DashAmount`) (`self.DashCount`))
      (`/Engine/EditorBlueprintResources/StandardMacros.IncrementInt` (`self.DashCount`)
        (:`  `
          (if (`self.InvincibleDash`)
            (if true
              (set `/Game/DamageSystem/BPC_PlayerDamagable.IsInvincible` true (`/Game/FirstPerson/Blueprints/BP_FirstPersonCharacter.BP_PlayerDamagable` _playerref))
              (`Character.LaunchCharacter` (`self.PlayerRef`) _returnvalue false false)
              (`KismetSystemLibrary.Delay` 0.6)
              (set `/Game/DamageSystem/BPC_PlayerDamagable.IsInvincible` false (`/Game/FirstPerson/Blueprints/BP_FirstPersonCharacter.BP_PlayerDamagable` (`self.PlayerRef`)))
              (set `self.DashCount` 0 :!label _label))
            (else
              (`Character.LaunchCharacter` (`self.PlayerRef`) _returnvalue false false)
              (`KismetSystemLibrary.Delay` 0.6)
              (goto _label))))))))

(event `Dash`
  (bind _playerref (`self.PlayerRef`))
  (bind _playerref_2 (`self.PlayerRef`))
  (bind (_playermod_typingtimemod _playermod_letterremoval _playermod_speedmod _playermod_dashmod) (break `/Game/Data/Structs/S_PlayerMods` (`/Game/FirstPerson/Blueprints/BP_FirstPersonCharacter.PlayerMod` _playerref_2)))
  (bind (_returnvalue_x _returnvalue_y) (`KismetMathLibrary.BreakVector` (`SceneComponent.GetForwardVector` (`/Game/FirstPerson/Blueprints/BP_FirstPersonCharacter.FirstPersonCamera` _playerref_2))))
  ;[0 0.05245 1] Dash Ability
  (if (> (`self.DashAmount`) (`self.DashCount`))
    (`/Engine/EditorBlueprintResources/StandardMacros.IncrementInt` (`self.DashCount`)
      (:`  `
        (if (`self.InvincibleDash`)
          (set `/Game/DamageSystem/BPC_PlayerDamagable.IsInvincible` true (`/Game/FirstPerson/Blueprints/BP_FirstPersonCharacter.BP_PlayerDamagable` _playerref)))
        (`Character.LaunchCharacter` _playerref (* (`KismetMathLibrary.MakeVector` _returnvalue_x _returnvalue_y) -3000.0 _playermod_dashmod) false false)
        (`KismetSystemLibrary.Delay` 0.6)
        (if (`self.InvincibleDash`)
          (set `/Game/DamageSystem/BPC_PlayerDamagable.IsInvincible` false (`/Game/FirstPerson/Blueprints/BP_FirstPersonCharacter.BP_PlayerDamagable` (`self.PlayerRef`)))
          (goto _label))))))

(event `EnhancedInput|/Game/FirstPerson/Input/Actions/IA_Stab`
  (params (ActionValue :type "Float (double-precision)") (ElapsedSeconds :type "Float (double-precision)") (TriggeredSeconds :type "Float (double-precision)") (InputAction :type "InputAction Object Reference" :default "/Game/FirstPerson/Input/Actions/IA_Stab.IA_Stab"))
  (bind _playerref (`self.PlayerRef`))
  (bind _returnvalue (`Actor.K2_GetActorLocation` _playerref))
  (bind (_playermod_typingtimemod _playermod_letterremoval _playermod_speedmod _playermod_dashmod _playermod_stabrangemod _playermod_stabdamagemod) (break `/Game/Data/Structs/S_PlayerMods` (`/Game/FirstPerson/Blueprints/BP_FirstPersonCharacter.PlayerMod` _playerref)))
  ;[0 0.05245 1] Stab
  (:`Started`
    (bind (_outhit _returnvalue_2) (`KismetSystemLibrary.SphereTraceSingle` :`Start` _returnvalue :`End` (+ _returnvalue (* (`SceneComponent.GetForwardVector` (`/Game/FirstPerson/Blueprints/BP_FirstPersonCharacter.FirstPersonCamera` _playerref)) 200.0 _playermod_stabrangemod)) :`TraceChannel` "TraceTypeQuery1" :`DrawDebugType` "ForDuration"))
    (if _returnvalue_2
      (bind _returnvalue_3 (`Actor.GetComponentByClass` (`.HitActor` (`GameplayStatics.BreakHitResult` _outhit)) "/Game/DamageSystem/BPC_Damagable.BPC_Damagable_C"))
      (`/Engine/EditorBlueprintResources/StandardMacros.IsValid` _returnvalue_3
        (:`Is Valid`
          (`/Game/DamageSystem/BPC_Damagable.Damaged` _returnvalue_3 (* 5.0 _playermod_stabdamagemod)))))))

(fn `KillChance`
  (bind _bp_playerdamagable (`/Game/FirstPerson/Blueprints/BP_FirstPersonCharacter.BP_PlayerDamagable` (`self.PlayerRef`)))
  ;[0 0.05245 1] Check Activation
  (bind _keys (`BlueprintMapLibrary.Map_Keys` (`self.KillActive`)))
  (for _array_element _keys
    (if (`BlueprintMapLibrary.Map_Find` (`self.KillActive`) _array_element)
      (switch `/Game/Data/E_KillBonuses` _array_element
        (:`NewEnumerator0`
          ;[0 0.05245 1] Health Up
          (if (<= (`KismetMathLibrary.RandomFloat`) 1.0)
            (set `/Game/DamageSystem/BPC_PlayerDamagable.Health` (+ (`/Game/DamageSystem/BPC_PlayerDamagable.Health` _bp_playerdamagable) (/ (`/Game/DamageSystem/BPC_PlayerDamagable.MaxHealth` _bp_playerdamagable) 10.0)) (`/Game/FirstPerson/Blueprints/BP_FirstPersonCharacter.BP_PlayerDamagable` (`self.PlayerRef`)))))
        (:`NewEnumerator1`
          ;[0 0.05245 1] Embold Player
          (if (<= (`KismetMathLibrary.RandomFloat`) 1.0)
            (`/Game/DamageSystem/BPC_GameEffects.TriggerBold` (`/Game/FirstPerson/Blueprints/BP_FirstPersonCharacter.BP_GameEffects` (`self.PlayerRef`)))))))))

(fn `PlayBonusChance`
  (bind _bp_playerdamagable (`/Game/FirstPerson/Blueprints/BP_FirstPersonCharacter.BP_PlayerDamagable` (`self.PlayerRef`)))
  ;[0 0.05245 1] Check Activation
  (bind _keys (`BlueprintMapLibrary.Map_Keys` (`self.PlayBonusActive`)))
  (for _array_element _keys
    (if (`BlueprintMapLibrary.Map_Find` (`self.PlayBonusActive`) _array_element)
      (switch `/Game/Data/E_PlayBonuses` _array_element
        (:`NewEnumerator0`
          ;[0 0.05245 1] Health Up
          (if (<= (`KismetMathLibrary.RandomFloat`) (`self.PlayWellBonus`))
            (set `/Game/DamageSystem/BPC_PlayerDamagable.Health` (+ (`/Game/DamageSystem/BPC_PlayerDamagable.Health` _bp_playerdamagable) (/ (`/Game/DamageSystem/BPC_PlayerDamagable.MaxHealth` _bp_playerdamagable) 10.0)) (`/Game/FirstPerson/Blueprints/BP_FirstPersonCharacter.BP_PlayerDamagable` (`self.PlayerRef`)))))
        (:`NewEnumerator1`
          ;[0 0.05245 1] Marks Up
          (if (<= (`KismetMathLibrary.RandomFloat`) (`self.PlayWellBonus`))
            (`/Game/FirstPerson/Blueprints/Economy/BPC_PlayerEconomy.AddMarks` (`/Game/FirstPerson/Blueprints/BP_FirstPersonCharacter.BPC_PlayerEconomy` (`self.PlayerRef`)) 5)))))))