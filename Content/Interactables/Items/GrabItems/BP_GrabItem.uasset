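; Base-style pickup actor that grants the player an active, passive or mod item and destroys itself on interaction.
; Its sphere overlap toggles the HUD interact widget and sets the first-person character's InteractCase, showing the prompt only while IsClosed is true.
; SelectClass hands active items to BPCGrabItem, otherwise constructs the passive or mod object, links mod items to that component and calls InitMessage with the player.
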(event OnComponentBeginOverlap(Sphere)
  (params (OverlappedComponent :type Primitive%20Component%20Object%20Reference) (OtherActor :type Actor%20Object%20Reference) (OtherComp :type Primitive%20Component%20Object%20Reference) (OtherBodyIndex :type Integer) (bFromSweep :type Boolean) (SweepResult :type Hit%20Result%20Structure%20%28by%20ref%29))
  ;[0 0.05245 1] Add Interact Widget
  (if (and (== OtherActor (Game|GetPlayerCharacter 0)) (Variables|Default|GetIsClosed?))
    (UserInterface|Viewport|AddtoViewport (Variables|/Game/Widgets/HUD/BP_HUD.BP_HUD_C|GetInteractRef (Variables|Default|GetHUDRef)) 0)
    (bind _asbp_first_person_character (Utilities|Casting|CastToBP_FirstPersonCharacter (Game|GetPlayerCharacter 0)))
    (Variables|/Game/FirstPerson/Blueprints/BP_FirstPersonCharacter.BP_FirstPersonCharacter_C|SetInteractCase _asbp_first_person_character 3)))

(event OnComponentEndOverlap(Sphere)
  (params (OverlappedComponent :type Primitive%20Component%20Object%20Reference) (OtherActor :type Actor%20Object%20Reference) (OtherComp :type Primitive%20Component%20Object%20Reference) (OtherBodyIndex :type Integer))
  ;[0 0.05245 1] Remove Interact Widget
  (if (== OtherActor (Game|GetPlayerCharacter 0))
    (Widget|RemovefromParent (Variables|/Game/Widgets/HUD/BP_HUD.BP_HUD_C|GetInteractRef (Variables|Default|GetHUDRef)))
    (bind _asbp_first_person_character (Utilities|Casting|CastToBP_FirstPersonCharacter (Game|GetPlayerCharacter 0)))
    (Variables|/Game/FirstPerson/Blueprints/BP_FirstPersonCharacter.BP_FirstPersonCharacter_C|SetInteractCase _asbp_first_person_character 0)))

(event EventBeginPlay
  ;[0 0.05245 1] Creates ref to HUD
  (bind _asbp_hud (Utilities|Casting|CastToBP_HUD (HUD|GetHUD (Game|GetPlayerController 0))))
  (Variables|Default|SetHUDRef _asbp_hud)
  (Variables|/Game/Interactables/Items/GrabItems/BPC_GrabItem.BPC_GrabItem_C|SetItemName (Variables|Default|GetBPC_GrabItem) (Variables|Default|GetItemName)))

(event EventInteraction
  (CallFunction|SelectClass)
  (Actor|DestroyActor))

(fn ConstructionScript)

(fn SelectClass
  (bind _item_info (Variables|Default|GetItem%20Info))
  (if (Utilities|IsValidClass (.activeblueprint _item_info))
    (Default|ActiveItem (Variables|Default|GetBPC_GrabItem) (Variables|Default|GetItem%20Info))
    (else
      (bind _returnvalue (Game|ConstructObjectfromClass (select (Utilities|IsValidClass (.passiveblueprint _item_info)) (.passiveblueprint _item_info) (.modblueprint _item_info))))
      (bind _asbp_mod_item (Utilities|Casting|CastToBP_ModItem _returnvalue)
        (:then
          (Variables|/Game/Interactables/Items/GrabItems/BP_ModItem.BP_ModItem_C|SetGrabItemRef _asbp_mod_item (Variables|Default|GetBPC_GrabItem)))
        (:CastFailed
          _))
      (bind _asbp_first_person_character (Utilities|Casting|CastToBP_FirstPersonCharacter (Game|Player|GetPlayerPawn 0)))
      (Class|BPICommitText|Init(Message) _returnvalue _asbp_first_person_character))))