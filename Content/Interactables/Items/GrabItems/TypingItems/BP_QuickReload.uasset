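; BP_QuickReload is a typing item whose committed command instantly refills the player's current weapon ammo.
; The refill runs only if CanCast is true after InkCheck, then updates the HUD ammo display.
; With the MoreToSay unique passive, reloading at or below a fifth of capacity, but not empty, overfills the weapon by an extra fifth.
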(event `self.CommandCommit`
  (bind _bp_weapon_component (`/Game/FirstPerson/Blueprints/BP_FirstPersonCharacter.BP_Weapon_Component` (`self.PlayerRef`)))
  (bind _currammo (`/Game/FirstPerson/Blueprints/Weapons/BPC_PlayerWeapon.CurrAmmo` _bp_weapon_component))
  (bind (_modinfo_weapontype _modinfo_ammo) (break `/Game/FirstPerson/Blueprints/Weapons/Mods/S_ModType` (`/Game/FirstPerson/Blueprints/Weapons/BPC_PlayerWeapon.ModInfo` _bp_weapon_component)))
  (bind _returnvalue (/ _modinfo_ammo 5))
  (`self.InkCheck`)
  (if (`self.Can Cast`)
    (if (and (`/Game/Interactables/Items/GrabItems/BPC_UniquePassives.MoreToSay` (`/Game/FirstPerson/Blueprints/BP_FirstPersonCharacter.BPC_UniquePassives` (`self.PlayerRef`))) (<= _currammo _returnvalue) (> _currammo 0))
      (set `/Game/FirstPerson/Blueprints/Weapons/BPC_PlayerWeapon.CurrAmmo` (+ _modinfo_ammo _returnvalue) _bp_weapon_component)
      (else
        (set `/Game/FirstPerson/Blueprints/Weapons/BPC_PlayerWeapon.CurrAmmo` _modinfo_ammo _bp_weapon_component)))
    (`/Game/Widgets/HUD/W_HUDOverlay.UpdateAmmo` (`/Game/Widgets/HUD/BP_HUD.HUDRef` (`/Game/FirstPerson/Blueprints/BP_FirstPersonCharacter.HudRef` (`self.PlayerRef`))))))