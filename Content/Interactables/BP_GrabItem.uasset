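; BP_GrabItem is a pickup actor that chooses its shop item in the construction script from the game instance's unlocked items.
; SelectItem picks randomly among DT_ShopItems rows matching SelectRarity's result, which is always one fixed tier because the weighted roll is disconnected.
; Sphere overlap toggles the HUD interact prompt and the player's InteractCase, showing it only while IsClosed is true.
; Interaction only destroys the actor, without granting the item here.
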(event `self.ReceiveBeginPlay`
  ;[0 0.05245 1] Creates ref to HUD
  (bind _asbp_hud (cast `/Game/Widgets/HUD/BP_HUD` (`PlayerController.GetHUD` (`GameplayStatics.GetPlayerController` 0))))
  (set `self.HUDRef` _asbp_hud))

(event `self.Sphere.OnComponentBeginOverlap`
  (params (OverlappedComponent :type "PrimitiveComponent Object Reference") (OtherActor :type "Actor Object Reference") (OtherComp :type "PrimitiveComponent Object Reference") (OtherBodyIndex :type Integer) (bFromSweep :type Boolean) (SweepResult :type "HitResult Structure (by ref)"))
  ;[0 0.05245 1] Add Interact Widget
  (if (and (== OtherActor (`GameplayStatics.GetPlayerCharacter` 0)) (`self.IsClosed?`))
    (`UserWidget.AddToViewport` (`/Game/Widgets/HUD/BP_HUD.InteractRef` (`self.HUDRef`)) 0)
    (bind _asbp_first_person_character (cast `/Game/FirstPerson/Blueprints/BP_FirstPersonCharacter` (`GameplayStatics.GetPlayerCharacter` 0)))
    (set `/Game/FirstPerson/Blueprints/BP_FirstPersonCharacter.InteractCase` 3 _asbp_first_person_character)))

(event `self.Sphere.OnComponentEndOverlap`
  (params (OverlappedComponent :type "PrimitiveComponent Object Reference") (OtherActor :type "Actor Object Reference") (OtherComp :type "PrimitiveComponent Object Reference") (OtherBodyIndex :type Integer))
  ;[0 0.05245 1] Remove Interact Widget
  (if (== OtherActor (`GameplayStatics.GetPlayerCharacter` 0))
    (`Widget.RemoveFromParent` (`/Game/Widgets/HUD/BP_HUD.InteractRef` (`self.HUDRef`)))
    (bind _asbp_first_person_character (cast `/Game/FirstPerson/Blueprints/BP_FirstPersonCharacter` (`GameplayStatics.GetPlayerCharacter` 0)))
    (set `/Game/FirstPerson/Blueprints/BP_FirstPersonCharacter.InteractCase` 0 _asbp_first_person_character)))

(event `/Game/Interactables/BPI_Interactable.Interaction`
  (`self.K2_DestroyActor`))

(fn `SelectItem`
  (params (Rarity :type "/Game/ShopSystem/E_ItemRarity Enum" :default "NewEnumerator0"))
  (returns (ItemInfo :type "/Game/ShopSystem/S_ItemInfo Structure"))
  (locals (PotentialItem :type "Array of Name"))
  (bind _asgi_player_stats (cast `/Game/SaveAndLoad/GI_PlayerStats` (`GameplayStatics.GetGameInstance`))
    (:`then`
      (for _array_element (`/Game/SaveAndLoad/GI_PlayerStats.UnlockedItems` _asgi_player_stats)
        (bind _returnvalue (`|GetDataTableRow` "/Game/ShopSystem/DT_ShopItems.DT_ShopItems" _array_element)
          (:`then`
            (if (`|EnumEquality` Rarity (`.Rarity_35_8A1D2B724F643BD098C4C7B1FED839D0` (break `/Game/ShopSystem/S_ItemInfo` _returnvalue)))
              (`KismetArrayLibrary.Array_AddUnique` (`local.PotentialItem`) _array_element)))))
      (bind _returnvalue_2 (`|GetDataTableRow` "/Game/ShopSystem/DT_ShopItems.DT_ShopItems" (`KismetArrayLibrary.Array_Random` (`local.PotentialItem`)))
        (:`then`
          (return _returnvalue_2))))
    (:`CastFailed`
      (`KismetSystemLibrary.PrintString` "Failed Game Instance"))))

(fn `SelectRarity`
  (returns (Rarity :type "/Game/ShopSystem/E_ItemRarity Enum"))
  (locals (Value :type "Float (double-precision)"))
  (return "NewEnumerator4"))

(fn `UserConstructionScript`
  (bind _rarity (`self.SelectRarity`))
  (bind _iteminfo (`self.SelectItem` _rarity))
  (bind _output_get (set `self.Item Info` _iteminfo))
  (`KismetSystemLibrary.PrintString` (`|GetEnumeratorNameAsString` (break `/Game/ShopSystem/S_ItemInfo` _output_get))))