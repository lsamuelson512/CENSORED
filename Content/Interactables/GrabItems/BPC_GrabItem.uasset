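; BPC_GrabItem is a component for grab items that applies stat modifiers to the player, their weapon and enemies.
; Each function adds the incoming struct onto the existing mods on the first-person character's weapon component, damagable component or PlayerMod, with Immunity combined by OR.
; Enemy mods accumulate on the BP_EnemySetter found in the world, which then runs Update.
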(fn `SetEnemyDamMod`
  (params (EnemyMod :type "/Game/DamageSystem/S_DamagableMods Structure"))
  (bind _returnvalue (`GameplayStatics.GetActorOfClass` "/Game/DamageSystem/BP_EnemySetter.BP_EnemySetter_C"))
  (bind (_enemymod_healthmod _enemymod_blockchance _enemymod_consumechance _enemymod_letterremoval _enemymod_revives _enemymod_immunity) (break `/Game/DamageSystem/S_DamagableMods` (`/Game/DamageSystem/BP_EnemySetter.EnemyMod` _returnvalue)))
  (set `/Game/DamageSystem/BP_EnemySetter.EnemyMod` (make `/Game/DamageSystem/S_DamagableMods` (+ _enemymod_healthmod EnemyMod_HealthMod_10_BAE72AAB47FDF15064B0CEB1E799FD82) (+ _enemymod_blockchance EnemyMod_BlockChance_33_3A9512E0453265518B6485A3E232D618) (+ _enemymod_consumechance EnemyMod_ConsumeChance_36_3AA448AE4DBCC37D284C2982F208618B) (+ _enemymod_letterremoval EnemyMod_LetterRemoval_30_C3D8DCB74527AB85D34429A9ACCFAEBF) 0 (or _enemymod_immunity EnemyMod_Immunity_14_51088F8647F1A26AA3E340B33C715AC5)) _returnvalue)
  (`/Game/DamageSystem/BP_EnemySetter.Update` _returnvalue))

(fn `SetPlayerDamMod`
  (params (Mods :type "/Game/DamageSystem/S_DamagableMods Structure"))
  (bind (_healthmod _blockchance _consumechance _letterremoval _revives _immunity) (break `/Game/DamageSystem/S_DamagableMods` Mods))
  (bind _asbp_first_person_character (cast `/Game/FirstPerson/Blueprints/BP_FirstPersonCharacter` (`GameplayStatics.GetPlayerPawn` 0)))
  (bind _bp_playerdamagable (`/Game/FirstPerson/Blueprints/BP_FirstPersonCharacter.BP_PlayerDamagable` _asbp_first_person_character))
  (bind (_mods_healthmod _mods_blockchance _mods_consumechance _mods_letterremoval _mods_revives _mods_immunity) (break `/Game/DamageSystem/S_DamagableMods` (`/Game/DamageSystem/BP_PlayerDamagable.Mods` _bp_playerdamagable)))
  (set `/Game/DamageSystem/BP_PlayerDamagable.Mods` (make `/Game/DamageSystem/S_DamagableMods` (+ _mods_healthmod _healthmod) (+ _mods_blockchance _blockchance) (+ _mods_consumechance _consumechance) (+ _mods_letterremoval _letterremoval) 0 (or _mods_immunity _immunity)) _bp_playerdamagable))

(fn `SetPlayerMod`
  (params (PlayerMod :type "/Game/DamageSystem/S_PlayerMods Structure"))
  (bind _asbp_first_person_character (cast `/Game/FirstPerson/Blueprints/BP_FirstPersonCharacter` (`GameplayStatics.GetPlayerPawn` 0)))
  (bind _playermod_typingtimemod (break `/Game/DamageSystem/S_PlayerMods` (`/Game/FirstPerson/Blueprints/BP_FirstPersonCharacter.PlayerMod` _asbp_first_person_character)))
  (set `/Game/FirstPerson/Blueprints/BP_FirstPersonCharacter.PlayerMod` (make `/Game/DamageSystem/S_PlayerMods` (+ _playermod_typingtimemod PlayerMod_TypingTimeMod_2_D66F9CFE42C8915A0AF8B48CE7CA515B)) _asbp_first_person_character))

(fn `SetWeaponMod`
  (params (DamagableMods :type "/Game/DamageSystem/S_WeaponMods Structure"))
  (bind _asbp_first_person_character (cast `/Game/FirstPerson/Blueprints/BP_FirstPersonCharacter` (`GameplayStatics.GetPlayerPawn` 0)))
  (bind _bp_weapon_component (`/Game/FirstPerson/Blueprints/BP_FirstPersonCharacter.BP_Weapon_Component` _asbp_first_person_character))
  (bind (_damagablemods_ammomod _damagablemods_damagemod _damagablemods_fireratemod) (break `/Game/DamageSystem/S_WeaponMods` (`/Game/FirstPerson/Blueprints/Weapons/BP_Weapon_Component.DamagableMods` _bp_weapon_component)))
  (set `/Game/FirstPerson/Blueprints/Weapons/BP_Weapon_Component.DamagableMods` (make `/Game/DamageSystem/S_WeaponMods` (+ _damagablemods_ammomod DamagableMods_AmmoMod_5_38F8A2EF405E66046BF5A0B5C51E918A) (+ _damagablemods_damagemod DamagableMods_DamageMod_9_80F6E31C4505A05798BFF9885A3215DA) (+ _damagablemods_fireratemod DamagableMods_FireRateMod_10_AB7D3E21446FAC1BF80BA8B3E29C53A2)) _bp_weapon_component))