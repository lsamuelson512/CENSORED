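; BP_BBDGrunt is a grunt enemy Blueprint with a health bar, damage handling and a weapon.
; On BeginPlay it sets the W_EnemyHealth widget's current and max health from BPDamagable's MaxHealth.
; Events spawn its default controller, pass effect and bold damage modifiers to BPEnemyWeapon, and forward underline damage to BPDamagable.
; The Strikethrough event calls PlayAnimMontage.
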(event `self.ReceiveBeginPlay`
  (bind _maxhealth (`/Game/DamageSystem/BPC_Damagable.MaxHealth` (`self.BP_Damagable`)))
  (bind _asw_enemy_health (cast `/Game/Widgets/Enemy/W_EnemyHealth` (`WidgetComponent.GetWidget` (`self.Healthbar`))))
  (set `/Game/Widgets/Enemy/W_EnemyHealth.Health` _maxhealth _asw_enemy_health)
  (set `/Game/Widgets/Enemy/W_EnemyHealth.MaxHealth` _maxhealth _asw_enemy_health))

(event `/Game/Enemies/BPI_EnemyActions.EnemyPosses`
  (`self.SpawnDefaultController`))

(event `/Game/DamageSystem/BPI_GameEffects.SetFxDamMod`
  (params (`Effect?` :type Boolean) (`Bold?` :type Boolean))
  (`/Game/Enemies/BP_EnemyWeapon.SetDamageMult` (`self.BP_EnemyWeapon`) `Effect?` `Bold?`))

(event `/Game/DamageSystem/BPI_GameEffects.UnderlineDamage`
  (`/Game/DamageSystem/BPC_Damagable.UnderlineDamage` (`self.BP_Damagable`)))

(event `/Game/DamageSystem/BPI_GameEffects.Strikethrough`
  (`self.PlayAnimMontage` null))

(fn `UserConstructionScript`)