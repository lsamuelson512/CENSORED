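; BPC_EnemyFunctions is an enemy component that switches the owner's AI sight perception off and back on.
; LosePerception disables the sight sense on the AI controller's perception component, forgets all perceived stimuli and clears the TargetActor blackboard key.
; RegainPerception waits for a given duration, then re-enables sight.
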(event `RegainPerception`
  (params (Duration :type "Float (single-precision)"))
  ;[0 0.05245 1] Enable Sensing
  (`KismetSystemLibrary.Delay` Duration)
  (`AIPerceptionComponent.SetSenseEnabled` (`Actor.GetComponentByClass` (`AIBlueprintHelperLibrary.GetAIController` (`self.GetOwner`)) "/Script/AIModule.AIPerceptionComponent") "/Script/AIModule.AISense_Sight" true))

(event `LosePerception`
  (bind _returnvalue (`self.GetOwner`))
  (bind _returnvalue_2 (`Actor.GetComponentByClass` (`AIBlueprintHelperLibrary.GetAIController` _returnvalue) "/Script/AIModule.AIPerceptionComponent"))
  ;[0 0.05245 1] Disabling Sensing
  (`AIPerceptionComponent.SetSenseEnabled` _returnvalue_2 "/Script/AIModule.AISense_Sight" false)
  (`AIPerceptionComponent.ForgetAll` _returnvalue_2)
  (`BlackboardComponent.SetValueAsObject` (`AIBlueprintHelperLibrary.GetBlackboard` _returnvalue) "TargetActor" null))