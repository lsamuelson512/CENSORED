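; Enemy projectile that damages the player or a decoy on hit and destroys itself on any impact.
; Only actors tagged Player take damage, via BPC_PlayerDamagable or, failing that, BPC_DecoyDamagable.
; Player damage also runs CheckEffects, which uses BulletMod to add Strikethrough build-up and roll chances for Italics and Underline on the victim's BPC_GameEffects; decoy hits skip these effects.
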(event `self.ReceiveHit`
  (params (MyComp :type "PrimitiveComponent Object Reference") (Other :type "Actor Object Reference") (OtherComp :type "PrimitiveComponent Object Reference") (bSelfMoved :type Boolean) (HitLocation :type "Vector Structure") (HitNormal :type "Vector Structure") (NormalImpulse :type "Vector Structure") (Hit :type "HitResult Structure (by ref)"))
  (bind _returnvalue (`self.GetComponentByClass` Other "/Game/DamageSystem/BPC_DecoyDamagable.BPC_DecoyDamagable_C"))
  (bind _returnvalue_2 (`self.GetComponentByClass` Other "/Game/DamageSystem/BPC_PlayerDamagable.BPC_PlayerDamagable_C"))
  (if (`self.ActorHasTag` Other "Player")
    (set `self.HitActor` Other)
    (`/Engine/EditorBlueprintResources/StandardMacros.IsValid` _returnvalue_2
      (:`Is Valid`
        (`/Game/DamageSystem/BPC_PlayerDamagable.Damaged` _returnvalue_2 (`self.Damage`))
        (`self.CheckEffects`)
        (`self.K2_DestroyActor` :!label _label) ; Then destroy this projectile
      )
      (:`Is Not Valid`
        (`/Engine/EditorBlueprintResources/StandardMacros.IsValid` _returnvalue
          (:`Is Valid`
            (`/Game/DamageSystem/BPC_PlayerDamagable.Damaged` _returnvalue (`self.Damage`))
            (goto _label))
          (:`Is Not Valid`
            (`self.K2_DestroyActor`)))))
    (else
      (`self.K2_DestroyActor`))))

(fn `CheckEffects`
  (bind (_bulletmod_strikethroughbuildup _bulletmod_italicsmod _bulletmod_underlinemod) (break `/Game/Data/Structs/S_BulletMods` (`self.BulletMod`)))
  (bind _returnvalue (`self.GetComponentByClass` (`self.HitActor`) "/Game/DamageSystem/BPC_GameEffects.BPC_GameEffects_C"))
  (`/Engine/EditorBlueprintResources/StandardMacros.IsValid` _returnvalue
    (:`Is Valid`
      (`/Game/DamageSystem/BPC_GameEffects.TriggerStrikethrough` _returnvalue _bulletmod_strikethroughbuildup)
      (if (<= (`KismetMathLibrary.RandomFloat`) _bulletmod_italicsmod)
        (`/Game/DamageSystem/BPC_GameEffects.TriggerItalics` _returnvalue))
      (if (<= (`KismetMathLibrary.RandomFloat`) _bulletmod_underlinemod)
        (`/Game/DamageSystem/BPC_GameEffects.TriggerUnderline` _returnvalue)))))

(fn `UserConstructionScript`)