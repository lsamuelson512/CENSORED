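; BP_D70 is a boss enemy character providing projectile, ground slam and teleport attacks, with dispatchers signaling when they end; kick combos are empty stubs.
; CalculateRoundPattern fires a 16-shot projectile ring, repeated with rotating yaw for the spinning attack.
; Ground slam launches the boss in an arc toward above the player, then sphere-traces for damage on landing.
; Teleport is a fast AI flight through pawns, adding side-fired lines or an arrival ring by health.
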(event `KickCombo1`)

(event `KickCombo2`)

(event `SpinningPattern`
  (bind _spinningcounter (`self.SpinningCounter`))
  ;[0 0.05245 1] Spinning Attack
  (if (<= _spinningcounter 35) :!label _label
    (`self.CalculateRoundPattern` (`KismetMathLibrary.MakeRotator` 0.0 0.0 (mod (* _spinningcounter 3.75) 135.0)))
    (bind _result (`/Engine/EditorBlueprintResources/StandardMacros.IncrementInt` (`self.SpinningCounter`))
      (:`  `
        (`KismetSystemLibrary.Delay` 0.1)
        (`KismetSystemLibrary.PrintString` (`KismetStringLibrary.Conv_IntToString` _result))
        (goto _label)))
    (else
      (set `self.SpinningCounter` 0)
      (`self.AttackEnd`))))

(event `OnLanding` :!signature `self.LandedDelegate`
  (params (Hit :type "HitResult Structure (by ref)"))
  (bind _returnvalue (`self.K2_GetActorLocation`))
  (bind _charactermovement (`self.CharacterMovement`))
  ;[0 0.05245 1] Ground Slam
  (remove `self.LandedDelegate` (delegate `OnLanding`))
  (bind _outhit (`KismetSystemLibrary.SphereTraceSingle` :`Start` _returnvalue :`End` _returnvalue :`Radius` 512.0 :`TraceChannel` "TraceTypeQuery1" :`DrawDebugType` "ForDuration"))
  (bind _returnvalue_2 (`self.GetComponentByClass` (`.HitActor` (`GameplayStatics.BreakHitResult` _outhit)) "/Game/DamageSystem/BPC_Damagable.BPC_Damagable_C"))
  (`/Engine/EditorBlueprintResources/StandardMacros.IsValid` _returnvalue_2
    (:`Is Valid`
      (`/Game/DamageSystem/BPC_Damagable.Damaged` _returnvalue_2 (stale `GroundSlam` DamageAmount)))
    (:`Is Not Valid`
      _))
  (`KismetSystemLibrary.Delay` 0.5)
  (`CharacterMovementComponent.SetMovementMode` _charactermovement "MOVE_Walking" 0)
  (set `CharacterMovementComponent.GravityScale` 1.0 _charactermovement)
  (`self.AttackEnd`))

(event `GroundSlam`
  (params (DamageAmount :type "Float (double-precision)"))
  ;[0 0.05245 1] Ground Slam
  (`CharacterMovementComponent.SetMovementMode` (`self.CharacterMovement`) "MOVE_Flying" 0)
  (bind _outlaunchvelocity (`GameplayStatics.SuggestProjectileVelocity_CustomArc` (`self.K2_GetActorLocation`) (+ (`self.K2_GetActorLocation` (`GameplayStatics.GetPlayerCharacter` 0)) (0.0 0.0 1000.0))))
  (`self.LaunchCharacter` _outlaunchvelocity true true)
  (add `self.LandedDelegate` (delegate `OnLanding`)))

(event `Teleport`
  (params (TargetActor :type "Actor Object Reference") (Health :type "Float (double-precision)"))
  (bind _charactermovement (`self.CharacterMovement`))
  ;[0 0.05245 1] Teleportation
  (if (< Health 75.0)
    (`self.ParallelPattern`))
  (`CharacterMovementComponent.SetMovementMode` _charactermovement "MOVE_Flying" 0)
  (set `CharacterMovementComponent.MaxFlySpeed` 2000.0 _charactermovement)
  (set `CharacterMovementComponent.MaxAcceleration` 99999.0 _charactermovement)
  (`PrimitiveComponent.SetCollisionResponseToChannel` (`self.CapsuleComponent`) "ECC_Pawn" "ECR_Ignore")
  (`|AIMoveTo` self (0.0 0.0 0.0) TargetActor
    (:`OnSuccess`
      _)
    (:`OnFail`
      _))
  (`self.ParallelStop`)
  (if (and (< Health 125.0) (> Health 75.0))
    (`self.RoundPattern`))
  (`self.TeleportEnd`))

(event `TeleportEnd`
  (bind _charactermovement (`self.CharacterMovement`))
  ;[0 0.05245 1] Teleportation
  (`CharacterMovementComponent.SetMovementMode` _charactermovement "MOVE_Walking" 0)
  (set `CharacterMovementComponent.MaxAcceleration` 2048.0 _charactermovement)
  (`PrimitiveComponent.SetCollisionResponseToChannel` (`self.CapsuleComponent`) "ECC_Pawn" "ECR_Block")
  (`self.OnTeleportEnd`))

(event `RoundPattern`
  ;[0 0.05245 1] Round Pattern
  (`self.CalculateRoundPattern` (struct)))

(event `ParallelPattern`
  (bind _returnvalue (`self.K2_GetActorLocation`))
  (bind (_returnvalue_roll _returnvalue_pitch _returnvalue_yaw) (`KismetMathLibrary.BreakRotator` (`self.K2_GetActorRotation`)))
  (bind _returnvalue_2 (`self.GetActorForwardVector`))
  ;[0 0.05245 1] Parallel Line Fire
  (set `self.ParallelLines?` true)
  (if (`self.ParallelLines?`) :!label _label_2
    (bind _returnvalue_3 (`|SpawnActorFromClass` "/Game/Enemies/BP_EnemyProjectile.BP_EnemyProjectile_C" (`KismetMathLibrary.MakeTransform` (+ _returnvalue (* (`KismetMathLibrary.GreaterGreater_VectorRotator` _returnvalue_2 (struct :`Yaw` -90.0)) 100.0)) (`KismetMathLibrary.MakeRotator` _returnvalue_roll _returnvalue_pitch (+ _returnvalue_yaw -90.0)) (5.0 5.0 5.0)) "Undefined" "MultiplyWithRoot" null (struct) null))
    (set `/Game/Enemies/BP_EnemyProjectile.Damage` 5.0 _returnvalue_3)
    (bind _returnvalue_4 (`|SpawnActorFromClass` "/Game/Enemies/BP_EnemyProjectile.BP_EnemyProjectile_C" (`KismetMathLibrary.MakeTransform` (+ _returnvalue (* (`KismetMathLibrary.GreaterGreater_VectorRotator` _returnvalue_2 (struct :`Yaw` 90.0)) 100.0)) (`KismetMathLibrary.MakeRotator` _returnvalue_roll _returnvalue_pitch (+ _returnvalue_yaw 90.0)) (5.0 5.0 5.0)) "Undefined" "MultiplyWithRoot" null (struct) null))
    (set `/Game/Enemies/BP_EnemyProjectile.Damage` 0.0 _returnvalue_4)
    (`KismetSystemLibrary.Delay` 0.15)
    (goto _label_2)))

(event `ParallelStop`
  ;[0 0.05245 1] Parallel Line Fire
  (set `self.ParallelLines?` false))

(fn `CalculateRoundPattern`
  (params (Deviation :type "Rotator Structure"))
  (locals (RotationBetweenShots :type "Rotator Structure" :default (struct :`Yaw` -90.0)))
  (bind _rotationbetweenshots (`local.RotationBetweenShots`))
  (for _ (range 16)
    (bind _returnvalue (`|SpawnActorFromClass` "/Game/Enemies/BP_EnemyProjectile.BP_EnemyProjectile_C" (`KismetMathLibrary.MakeTransform` (+ (`self.K2_GetActorLocation`) (* (`KismetMathLibrary.GreaterGreater_VectorRotator` (`self.GetActorForwardVector`) _rotationbetweenshots) 100.0)) (`KismetMathLibrary.ComposeRotators` (`KismetMathLibrary.ComposeRotators` (`self.K2_GetActorRotation`) _rotationbetweenshots) Deviation) (5.0 5.0 5.0)) "Undefined" "MultiplyWithRoot" null (struct) null))
    (set `/Game/Enemies/BP_EnemyProjectile.Damage` 5.0 _returnvalue)
    (set `local.RotationBetweenShots` (`KismetMathLibrary.ComposeRotators` (`local.RotationBetweenShots`) (struct :`Yaw` 22.5)))))

(fn `UserConstructionScript`
  (`parent.UserConstructionScript`))