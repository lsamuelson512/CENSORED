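; Boss enemy character that can spawn its default controller on demand and perform a teleport-style move to a target actor.
; The teleport is a very fast flight via AI MoveTo, with boosted acceleration and pawn collision ignored.
; On either success or failure, TeleportEnd restores walking, acceleration and pawn blocking, then fires the OnTeleportEnd dispatcher.
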(event `self.EnemyPosses`
  (`self.SpawnDefaultController`))

(event `Teleport`
  (params (TargetActor :type "Actor Object Reference"))
  (bind _charactermovement (`self.CharacterMovement`))
  (`CharacterMovementComponent.SetMovementMode` _charactermovement "MOVE_Flying" 0)
  (set `CharacterMovementComponent.MaxFlySpeed` 5000.0 _charactermovement)
  (set `CharacterMovementComponent.MaxAcceleration` 99999.0 _charactermovement)
  (`PrimitiveComponent.SetCollisionResponseToChannel` (`self.CapsuleComponent`) "ECC_Pawn" "ECR_Ignore")
  (`|AIMoveTo` self (0.0 0.0 0.0) TargetActor
    (:`OnSuccess`
      _)
    (:`OnFail`
      _))
  (`self.TeleportEnd`))

(event `TeleportEnd`
  (bind _charactermovement (`self.CharacterMovement`))
  (`CharacterMovementComponent.SetMovementMode` _charactermovement "MOVE_Walking" 0)
  (set `CharacterMovementComponent.MaxAcceleration` 2048.0 _charactermovement)
  (`PrimitiveComponent.SetCollisionResponseToChannel` (`self.CapsuleComponent`) "ECC_Pawn" "ECR_Block")
  (`self.OnTeleportEnd`))

(fn `UserConstructionScript`)